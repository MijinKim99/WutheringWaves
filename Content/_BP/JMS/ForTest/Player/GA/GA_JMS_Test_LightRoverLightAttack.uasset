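; Test gameplay ability for LightRover's ground light-attack combo, handing off to the air attack ability when airborne.
; It shows the sword, turns toward camera-relative input and plays the current combo montage, advancing or wrapping the character's combo count.
; A hit-start event briefly delays spawning a pooled weapon-socket hitbox with light, stagger and parry damage, deactivated by hit-end.
; Montage end hides the sword and starts a short combo-reset timer, cleared by the next attack.
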(event `self.K2_ActivateAbility`
  (bind _returnvalue (`self.GetPlayerCharacterFromActorInfo`))
  (if (`PlayerCharacter.bIsGrounded` (`self.GetPlayerCharacterFromActorInfo`))
    ;[1 1 1] 공중공격을 구현해야하기에, 애니메이션 캔슬되는 거 놔둠
    (`self.VisibleWeapon`)
    (`self.RotateMoveDirection`)
    (`KismetSystemLibrary.K2_ClearAndInvalidateTimerHandle` (`self.ResetTimerHandle`))
    (set `self.CachedComboCount` (`PlayerCharacter.LightAttackComboCount` (`self.GetPlayerCharacterFromActorInfo`)))
    (`AbilityTask_PlayMontageAndWait.CreatePlayMontageAndWaitProxy` "None" (`BlueprintMapLibrary.Map_Find` (`self.AttackMontageMap`) (`PlayerCharacter.LightAttackComboCount` (`self.GetPlayerCharacterFromActorInfo`)))
      (:`then`
        (`|ExecutionSequence`
          (:`then_0`
            (if (== (`PlayerCharacter.LightAttackComboCount` (`self.GetPlayerCharacterFromActorInfo`)) (`BlueprintMapLibrary.Map_Length` (`self.AttackMontageMap`)))
              (`self.ResetComboCount`)
              (else
                (`/Engine/EditorBlueprintResources/StandardMacros.IncrementInt` (`PlayerCharacter.LightAttackComboCount` (`self.GetPlayerCharacterFromActorInfo`))))))
          (:`then_1`
            (set `PlayerCharacter.bAttackMode` true _returnvalue)
            (set `PlayerCharacter.bSprintMode` false _returnvalue))
          (:`then_2`
            (`AbilityTask_WaitGameplayEvent.WaitGameplayEvent` (struct :`TagName` "Player.Event.HitEnemy.Start") null
              (:`EventReceived`
                (`KismetSystemLibrary.K2_SetTimerDelegate` (delegate `OnGroundAttackCollision`) 0.05))))))
      (:`OnCompleted`
        (`self.K2_EndAbility` :!label _label)
        (bind _returnvalue_2 (`KismetSystemLibrary.K2_SetTimerDelegate` (delegate `ResetComboCount`) 0.25))
        (set `self.ResetTimerHandle` _returnvalue_2))
      (:`OnBlendOut`
        (goto _label))
      (:`OnInterrupted`
        (goto _label))
      (:`OnCancelled`
        (goto _label)))
    (else
      (`AbilitySystemComponent.TryActivateAbilityByClass` (`self.GetWWAbilitySystemComponentFromActorInfo`) "/Game/_BP/YHG/Characters/LightRover/GA/GA_LightRoverAirAttack.GA_LightRoverAirAttack_C" true)
      (`self.K2_EndAbility`))))

(event `self.K2_OnEndAbility`
  (params (bWasCancelled :type Boolean))
  (`self.HiddenWeapon`))

(event `OnGroundAttackCollision`
  (bind _asbp_jms_test_player_character (cast `/Game/_BP/JMS/ForTest/Player/BP_JMS_TestPlayerCharacter` (`self.GetPlayerCharacterFromActorInfo`)))
  (bind _returnvalue (`WWObjectPoolComponent.SpawnPooledObject` (`/Game/_BP/JMS/ForTest/Player/BP_JMS_TestPlayerCharacter.LightAttackCollision` _asbp_jms_test_player_character) _asbp_jms_test_player_character))
  (bind _asattack_collision_box (cast `AttackCollisionBox` _returnvalue))
  (`AttackCollisionBox.InitializeAttachedBoxAndAttackMultipleEffects` :`self` _asattack_collision_box :`BoxExtent` (100.0 100.0 100.0) :`InstigatorMesh` (`self.GetOwningComponentFromActorInfo`) :`AttachSocketName` "WeaponProp02" :`InGameplayEffectSpecHandles` (`|MakeArray` (`self.MakePlayerDamageGameplayEffectSpecHandle` "/Game/_BP/JMS/Character/AbilitySystem/GE/GE_Damaged_Enemy.GE_Damaged_Enemy_C" 10.0 (struct :`TagName` "Shared.SetByCaller.Damage.Light")) (`self.MakePlayerDamageGameplayEffectSpecHandle` "/Game/_BP/JMS/Character/AbilitySystem/GE/GE_Damaged_Enemy.GE_Damaged_Enemy_C" 15.0 (struct :`TagName` "Shared.SetByCaller.Damage.Stagger")) (`self.MakePlayerDamageGameplayEffectSpecHandle` "/Game/_BP/JMS/Character/AbilitySystem/GE/GE_Damaged_Enemy.GE_Damaged_Enemy_C" 20.0 (struct :`TagName` "Shared.SetByCaller.Damage.Parry"))) :`InHitReactEventTag` (struct :`TagName` "Shared.Event.HitReact.Small") :`bShowCollisionInGame` true)
  (`AbilityTask_WaitGameplayEvent.WaitGameplayEvent` (struct :`TagName` "Player.Event.HitEnemy.End") null
    (:`EventReceived`
      (`AttackCollisionBox.DeactivateIfActivated` _asattack_collision_box))))

(event `ResetComboCount`
  (set `PlayerCharacter.LightAttackComboCount` 1 (`self.GetPlayerCharacterFromActorInfo`)))

(fn `GroundAttackDamage`)

(fn `HiddenWeapon`
  (bind _asbp_light_rover_character (cast `/Game/_BP/YHG/Characters/LightRover/BP_LightRoverCharacter` (`self.GetPlayerCharacterFromActorInfo`)))
  (`SceneComponent.SetVisibility` (`/Game/_BP/YHG/Characters/LightRover/BP_LightRoverCharacter.Scabbard` _asbp_light_rover_character) false false)
  (`SceneComponent.SetVisibility` (`/Game/_BP/YHG/Characters/LightRover/BP_LightRoverCharacter.Sword` _asbp_light_rover_character) false false))

(fn `RotateMoveDirection`
  (bind _followcamera (`PlayerCharacter.FollowCamera` (`self.GetPlayerCharacterFromActorInfo`)))
  (bind (_returnvalue_x _returnvalue_y) (`KismetMathLibrary.BreakVector` (`SceneComponent.GetRightVector` _followcamera)))
  (bind (_x _y) (`KismetMathLibrary.BreakVector2D` (`WWPlayerController.IsInputMove` (`self.GetPlayerControllerFromActorInfo`))))
  (bind (_returnvalue_x_2 _returnvalue_y_2) (`KismetMathLibrary.BreakVector` (`SceneComponent.GetForwardVector` _followcamera)))
  (bind _returnvalue (+ (* (`KismetMathLibrary.Normal` (`KismetMathLibrary.MakeVector` _returnvalue_x _returnvalue_y)) _x) (* (`KismetMathLibrary.Normal` (`KismetMathLibrary.MakeVector` _returnvalue_x_2 _returnvalue_y_2)) _y)))
  (if (`KismetMathLibrary.NotEqualExactly_VectorVector` _returnvalue)
    (`Actor.K2_SetActorRotation` (`self.GetPlayerCharacterFromActorInfo`) (`KismetMathLibrary.MakeRotFromX` _returnvalue) true)))

(fn `VisibleWeapon`
  (bind _asbp_light_rover_character (cast `/Game/_BP/YHG/Characters/LightRover/BP_LightRoverCharacter` (`self.GetPlayerCharacterFromActorInfo`)))
  (`SceneComponent.SetVisibility` (`/Game/_BP/YHG/Characters/LightRover/BP_LightRoverCharacter.Scabbard` _asbp_light_rover_character) true false)
  (`SceneComponent.SetVisibility` (`/Game/_BP/YHG/Characters/LightRover/BP_LightRoverCharacter.Sword` _asbp_light_rover_character) true false))