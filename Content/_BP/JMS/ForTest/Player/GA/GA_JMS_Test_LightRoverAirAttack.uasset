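; Test gameplay ability for the LightRover player's light air attack, a montage-driven plunge that deals area damage on landing.
; On activation it hides the sword and scabbard, faces camera-relative input, resets the combo count and binds a landed delegate.
; Landing on an enemy briefly ignores Pawn collision to pass through.
; Landing elsewhere jumps to the end section and, after a short delay, spawns a pooled box hitbox applying light damage.
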(event `self.K2_ActivateAbility`
  (`self.K2_CommitAbilityCost` false)
  (`self.HiddenWeapon`)
  (`self.RotateMoveDirection`)
  (`self.ResetComboCount`)
  (`AbilityTask_PlayMontageAndWait.CreatePlayMontageAndWaitProxy` "None" "/Game/_BP/YHG/Characters/LightRover/Animation/UseAnimation/CharacterAnim/Attack/AM_LightRoverAnim_R2T1PlayerMaleMd10011_Lod4_AirAttack_Edited.AM_LightRoverAnim_R2T1PlayerMaleMd10011_Lod4_AirAttack_Edited"
    (:`then`
      (add `Character.LandedDelegate` (`self.GetPlayerCharacterFromActorInfo`) (delegate `LandedDelegate_Event`)))
    (:`OnCompleted`
      (`self.K2_EndAbility` :!label _label))
    (:`OnBlendOut`
      (goto _label))
    (:`OnInterrupted`
      (goto _label))
    (:`OnCancelled`
      (goto _label))))

(event `LandedDelegate_Event`
  (params (Hit :type "HitResult Structure (by ref)"))
  (cast `EnemyCharacter` Hit_HitActor
    (:`then`
      (`PrimitiveComponent.SetCollisionResponseToChannel` (`Character.CapsuleComponent` (`self.GetPlayerCharacterFromActorInfo`)) "ECC_Pawn" "ECR_Ignore")
      (`KismetSystemLibrary.K2_SetTimerDelegate` (delegate `OnCollisionResponseToEnemy`) 0.05))
    (:`CastFailed`
      (`self.MontageJumpToSection` "AirAttackEnd")
      (`KismetSystemLibrary.K2_SetTimerDelegate` (delegate `OnAirAttackCollision`) 0.05)
      (clear `Character.LandedDelegate` (`self.GetPlayerCharacterFromActorInfo`)))))

(event `ResetComboCount`
  (set `PlayerCharacter.LightAttackComboCount` 1 (`self.GetPlayerCharacterFromActorInfo`)))

(event `OnCollisionResponseToEnemy`
  (`PrimitiveComponent.SetCollisionResponseToChannel` (`Character.CapsuleComponent` (`self.GetPlayerCharacterFromActorInfo`)) "ECC_Pawn" "ECR_Block"))

(event `OnAirAttackCollision`
  (`self.AirAttackDamage`))

(fn `AirAttackDamage`
  (bind _asbp_light_rover_character (cast `/Game/_BP/YHG/Characters/LightRover/BP_LightRoverCharacter` (`self.GetPlayerCharacterFromActorInfo`)))
  (bind _returnvalue (`WWObjectPoolComponent.SpawnPooledObject` (`/Game/_BP/YHG/Characters/LightRover/BP_LightRoverCharacter.LightAttackCollision` _asbp_light_rover_character) _asbp_light_rover_character))
  (bind _asbp_light_rover_light_attack_collision (cast `/Game/_BP/YHG/Characters/LightRover/AttackCollisionBP/BP_LightRoverLightAttackCollision` _returnvalue))
  (`AttackCollisionBox.InitializeAndAttackWithBox` :`self` _asbp_light_rover_light_attack_collision :`Duration` 0.1 :`BoxExtent` (128.0 128.0 128.0) :`Location` (+ (`Actor.K2_GetActorLocation` _asbp_light_rover_character) (* (`Actor.GetActorUpVector` _asbp_light_rover_character) 16.0)) :`InGameplayEffectSpecHandle` (`self.MakePlayerDamageGameplayEffectSpecHandle` "/Game/_BP/JMS/Character/AbilitySystem/GE/GE_Damaged_Enemy.GE_Damaged_Enemy_C" 50.0 (struct :`TagName` "Shared.SetByCaller.Damage.Light"))))

(fn `HiddenWeapon`
  (bind _asbp_light_rover_character (cast `/Game/_BP/YHG/Characters/LightRover/BP_LightRoverCharacter` (`self.GetPlayerCharacterFromActorInfo`)))
  (`SceneComponent.SetVisibility` (`/Game/_BP/YHG/Characters/LightRover/BP_LightRoverCharacter.Scabbard` _asbp_light_rover_character) false false)
  (`SceneComponent.SetVisibility` (`/Game/_BP/YHG/Characters/LightRover/BP_LightRoverCharacter.Sword` _asbp_light_rover_character) false false))

(fn `RotateMoveDirection`
  (bind _followcamera (`PlayerCharacter.FollowCamera` (`self.GetPlayerCharacterFromActorInfo`)))
  (bind (_returnvalue_x _returnvalue_y) (`KismetMathLibrary.BreakVector` (`SceneComponent.GetRightVector` _followcamera)))
  (bind (_x _y) (`KismetMathLibrary.BreakVector2D` (`WWPlayerController.IsInputMove` (`self.GetPlayerControllerFromActorInfo`))))
  (bind (_returnvalue_x_2 _returnvalue_y_2) (`KismetMathLibrary.BreakVector` (`SceneComponent.GetForwardVector` _followcamera)))
  (bind _returnvalue (+ (* (`KismetMathLibrary.Normal` (`KismetMathLibrary.MakeVector` _returnvalue_x _returnvalue_y)) _x) (* (`KismetMathLibrary.Normal` (`KismetMathLibrary.MakeVector` _returnvalue_x_2 _returnvalue_y_2)) _y)))
  (if (`KismetMathLibrary.NotEqualExactly_VectorVector` _returnvalue)
    (`Actor.K2_SetActorRotation` (`self.GetPlayerCharacterFromActorInfo`) (`KismetMathLibrary.MakeRotFromX` _returnvalue) true)))