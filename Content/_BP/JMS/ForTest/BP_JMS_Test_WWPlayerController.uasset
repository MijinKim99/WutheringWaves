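; Test player controller that turns Enhanced Input into movement and briefly pulsed action flags, and switches possession between LightRover, Chixia and Verina, tagging PlayerState with the active one.
; A looping timer finds the nearest nearby enemy, retargeting only without a valid target or when dashing with movement input.
; It also loads weapon inventory from a DataTable, handles equip ownership, shows the level-timer HUD, and opens pausing character and inventory menus.
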(event `EnhancedInput|/Game/_BP/YHG/Inputs/Actions/IA_Move`
  (params (ActionValue :type "Vector2D Structure") (ElapsedSeconds :type "Float (double-precision)") (TriggeredSeconds :type "Float (double-precision)") (InputAction :type "InputAction Object Reference" :default "/Game/_BP/YHG/Inputs/Actions/IA_Move.IA_Move"))
  (:`Triggered`
    (set `self.IsInputMove` ActionValue))
  (:`Completed`
    (set `self.IsInputMove` (0.0 0.0))))

(event `EnhancedInput|/Game/_BP/YHG/Inputs/Actions/IA_Dash`
  (params (ActionValue :type Boolean) (ElapsedSeconds :type "Float (double-precision)") (TriggeredSeconds :type "Float (double-precision)") (InputAction :type "InputAction Object Reference" :default "/Game/_BP/YHG/Inputs/Actions/IA_Dash.IA_Dash"))
  (:`Started`
    (set `self.bIsInputDash` true)
    (`KismetSystemLibrary.Delay` 0.05)
    (set `self.bIsInputDash` false)))

(event `EnhancedInput|/Game/_BP/YHG/Inputs/Actions/IA_Jump`
  (params (ActionValue :type Boolean) (ElapsedSeconds :type "Float (double-precision)") (TriggeredSeconds :type "Float (double-precision)") (InputAction :type "InputAction Object Reference" :default "/Game/_BP/YHG/Inputs/Actions/IA_Jump.IA_Jump"))
  (:`Started`
    (set `self.bIsInputJump` true)
    (`KismetSystemLibrary.Delay` 0.05)
    (set `self.bIsInputJump` false)))

(event `EnhancedInput|/Game/_BP/YHG/Inputs/Actions/IA_LightAttack`
  (params (ActionValue :type Boolean) (ElapsedSeconds :type "Float (double-precision)") (TriggeredSeconds :type "Float (double-precision)") (InputAction :type "InputAction Object Reference" :default "/Game/_BP/YHG/Inputs/Actions/IA_LightAttack.IA_LightAttack"))
  (:`Started`
    (set `self.bIsInputLightAttack` true)
    (`KismetSystemLibrary.Delay` 0.05)
    (set `self.bIsInputLightAttack` false)))

(event `EnhancedInput|/Game/_BP/YHG/Inputs/Actions/IA_Character1`
  (params (ActionValue :type Boolean) (ElapsedSeconds :type "Float (double-precision)") (TriggeredSeconds :type "Float (double-precision)") (InputAction :type "InputAction Object Reference" :default "/Game/_BP/YHG/Inputs/Actions/IA_Character1.IA_Character1"))
  (:`Started`
    (bind _returnvalue (`GameplayStatics.GetActorOfClass` "/Game/_BP/YHG/Characters/LightRover/BP_LightRoverCharacter.BP_LightRoverCharacter_C"))
    (`/Engine/EditorBlueprintResources/StandardMacros.IsValid` _returnvalue
      (:`Is Valid`
        (if (!= _returnvalue (`self.ControlledPlayerCharacter`))
          (`self.Possess` _returnvalue)
          (`SkeletalMeshComponent.SetAnimInstanceClass` (`Character.Mesh` _returnvalue) "/Game/_BP/YHG/Characters/LightRover/Animation/ABP_LightRoverAnim.ABP_LightRoverAnim_C"))))))

(event `EnhancedInput|/Game/_BP/YHG/Inputs/Actions/IA_Character2`
  (params (ActionValue :type Boolean) (ElapsedSeconds :type "Float (double-precision)") (TriggeredSeconds :type "Float (double-precision)") (InputAction :type "InputAction Object Reference" :default "/Game/_BP/YHG/Inputs/Actions/IA_Character2.IA_Character2"))
  (:`Started`
    (bind _returnvalue (`GameplayStatics.GetActorOfClass` "/Game/_BP/YHG/Characters/Chixia/BP_ChixiaCharacter.BP_ChixiaCharacter_C"))
    (`/Engine/EditorBlueprintResources/StandardMacros.IsValid` _returnvalue
      (:`Is Valid`
        (if (!= _returnvalue (`self.ControlledPlayerCharacter`))
          (`self.Possess` _returnvalue)
          (`SkeletalMeshComponent.SetAnimInstanceClass` (`Character.Mesh` _returnvalue) "/Game/_BP/YHG/Characters/Chixia/Animation/ABP_ChixiaAnim.ABP_ChixiaAnim_C"))))))

(event `EnhancedInput|/Game/_BP/YHG/Inputs/Actions/IA_Character3`
  (params (ActionValue :type Boolean) (ElapsedSeconds :type "Float (double-precision)") (TriggeredSeconds :type "Float (double-precision)") (InputAction :type "InputAction Object Reference" :default "/Game/_BP/YHG/Inputs/Actions/IA_Character3.IA_Character3"))
  (:`Started`
    (bind _returnvalue (`GameplayStatics.GetActorOfClass` "/Game/_BP/YHG/Characters/Verina/BP_VerinaCharacter.BP_VerinaCharacter_C"))
    (`/Engine/EditorBlueprintResources/StandardMacros.IsValid` _returnvalue
      (:`Is Valid`
        (if (!= _returnvalue (`self.ControlledPlayerCharacter`))
          (`self.Possess` _returnvalue)
          (`SkeletalMeshComponent.SetAnimInstanceClass` (`Character.Mesh` _returnvalue) "/Game/_BP/YHG/Characters/Verina/Animation/ABP_VerinaAnim.ABP_VerinaAnim_C"))))))

(event `self.ReceivePossess`
  (params (PossessedPawn :type "Pawn Object Reference"))
  (bind _playerstate (`self.PlayerState`))
  (bind _playerstate_2 (`self.PlayerState`))
  (bind _playerstate_3 (`self.PlayerState`))
  (set `self.Possessed Pawn` PossessedPawn)
  (`|ExecutionSequence`
    (:`then_0`
      (cast `/Game/_BP/YHG/Characters/LightRover/BP_LightRoverCharacter` (`self.Possessed Pawn`))
      (`WWBlueprintFunctionLibrary.AddTagToActor` _playerstate_3 (struct :`TagName` "Player.Status.PlayingCharacter.LightRover"))
      (`WWBlueprintFunctionLibrary.RemoveTagFromActor` _playerstate_3 (struct :`TagName` "Player.Status.PlayingCharacter.Chixia"))
      (`WWBlueprintFunctionLibrary.RemoveTagFromActor` _playerstate_3 (struct :`TagName` "Player.Status.PlayingCharacter.Verina")))
    (:`then_1`
      (cast `/Game/_BP/YHG/Characters/Chixia/BP_ChixiaCharacter` (`self.Possessed Pawn`))
      (`WWBlueprintFunctionLibrary.AddTagToActor` _playerstate_2 (struct :`TagName` "Player.Status.PlayingCharacter.Chixia"))
      (`WWBlueprintFunctionLibrary.RemoveTagFromActor` _playerstate_2 (struct :`TagName` "Player.Status.PlayingCharacter.LightRover"))
      (`WWBlueprintFunctionLibrary.RemoveTagFromActor` _playerstate_2 (struct :`TagName` "Player.Status.PlayingCharacter.Verina")))
    (:`then_2`
      (cast `/Game/_BP/YHG/Characters/Verina/BP_VerinaCharacter` (`self.Possessed Pawn`))
      (`WWBlueprintFunctionLibrary.AddTagToActor` _playerstate (struct :`TagName` "Player.Status.PlayingCharacter.Verina"))
      (`WWBlueprintFunctionLibrary.RemoveTagFromActor` _playerstate (struct :`TagName` "Player.Status.PlayingCharacter.LightRover"))
      (`WWBlueprintFunctionLibrary.RemoveTagFromActor` _playerstate (struct :`TagName` "Player.Status.PlayingCharacter.Chixia")))))

(event `self.ReceiveUnPossess`
  (params (UnpossessedPawn :type "Pawn Object Reference")))

(event `self.ReceiveBeginPlay`
  (`KismetSystemLibrary.K2_SetTimer` null "FindClosestEnemy" 0.1 true)
  (`KismetArrayLibrary.Array_Clear` (`self.Inventory_Weapon`))
  (bind _outrownames (`DataTableFunctionLibrary.GetDataTableRowNames` "/Game/_BP/KMJ/DataTable/Weapons/DT_Inventory_Weapon.DT_Inventory_Weapon"))
  (for _array_element _outrownames
    (bind _returnvalue (`|GetDataTableRow` "/Game/_BP/KMJ/DataTable/Weapons/DT_Inventory_Weapon.DT_Inventory_Weapon" _array_element)
      (:`then`
        (`KismetArrayLibrary.Array_Add` (`self.Inventory_Weapon`) _returnvalue))))
  (bind _returnvalue_2 (`|CreateWidget` "/Game/_BP/JMS/TowerBattleSystem/LevelUI/WBP_JMS_Test_PlayerHUD_Tower.WBP_JMS_Test_PlayerHUD_Tower_C"))
  (bind _output_get (set `self.Widget_JMS_Test_PlayerHUD_Tower` _returnvalue_2))
  (bind _returnvalue_3 (`GameplayStatics.GetActorOfClass` "/Script/WutheringWaves.WWLevelTimer"))
  (add `WWLevelTimer.OnTimerUpdate` _returnvalue_3 (delegate `OnTimerUpdate_Event`))
  (`UserWidget.AddToViewport` _output_get 0)
  (`/Game/_BP/JMS/TowerBattleSystem/LevelUI/WBP_JMS_Test_PlayerHUD_Tower.SetTimerUIEnabled` _output_get true))

(event `self.ChangeWeapon`
  (params (PreviousWeapon :type "Inventory_Weapon Structure") (NewWeapon :type "Inventory_Weapon Structure") (Index :type Integer))
  (`self.ChangeEquippedWeapon` PreviousWeapon NewWeapon Index))

(event `OnTimerUpdate_Event`
  (params (NewTime :type "Float (single-precision)"))
  (`/Game/_BP/JMS/TowerBattleSystem/LevelUI/WBP_JMS_Test_PlayerHUD_Tower.UpdateTimer` (`self.Widget_JMS_Test_PlayerHUD_Tower`) NewTime))

(event `Key|C`
  (params (Key :type "Key Structure"))
  (:`Pressed`
    (`/Game/_BP/KMJ/Widget/CharacterSetting/BP_CharSettingUIComponent.CreateWidget_CharSetting` (`self.BP_CharSettingUIComponent`))
    (`Widget.SetVisibility` (`self.Widget_PlayerHUD`) "Hidden")
    (`GameplayStatics.SetGamePaused` true)
    (set `self.bShowMouseCursor` true)))

(event `Key|B`
  (params (Key :type "Key Structure"))
  (:`Pressed`
    (`/Game/_BP/KMJ/Widget/CharacterSetting/BP_CharSettingUIComponent.CreateWidget_Inventory` (`self.BP_CharSettingUIComponent`))
    (`GameplayStatics.SetGamePaused` true)))

(event `self.ReceiveTick`
  (params (DeltaSeconds :type "Float (single-precision)"))
  (`KismetSystemLibrary.PrintString` (`KismetSystemLibrary.GetDisplayName` (`self.ClosestEnemy`)) true true (struct :`G` 0.66 :`B` 1.0 :`A` 1.0) 2.0 "ClosestEnemy"))

(fn `ChangeEquippedWeapon`
  (params (PreviousWeapon :type "Inventory_Weapon Structure") (NewWeapon :type "Inventory_Weapon Structure") (Index :type Integer))
  (bind (_weaponcurrentlevel _weaponcurrentrank _skillrank _itemowner _itemownerimage _rowindex) (break `Inventory_Weapon` NewWeapon))
  (bind (_weaponcurrentlevel_2 _weaponcurrentrank_2 _skillrank_2 _itemowner_2 _itemownerimage_2) (break `Inventory_Weapon` PreviousWeapon))
  ;[0.2969 0.2969 0.2969] 무기 장착 해제
  (for (_array_element _array_index) (`self.Inventory_Weapon`)
    (bind (_weaponcurrentlevel_3 _weaponcurrentrank_3 _skillrank_3 _itemowner_3 _itemownerimage_3 _rowindex_2) (break `Inventory_Weapon` _array_element))
    (if (`|EnumEquality` _itemowner_3 _itemowner_2)
      (`KismetArrayLibrary.Array_Set` (`self.Inventory_Weapon`) _array_index (make `Inventory_Weapon` _weaponcurrentlevel_3 _weaponcurrentrank_3 _skillrank_3 "None" _itemownerimage_3 _rowindex_2))
      (break)))
  ;[0.2708 0.2708 0.2708] 무기 새로 장착
  (for (_ _array_index_2) (`self.Inventory_Weapon`)
    (if (== Index _array_index_2)
      (`KismetArrayLibrary.Array_Set` (`self.Inventory_Weapon`) _array_index_2 (make `Inventory_Weapon` _weaponcurrentlevel _weaponcurrentrank _skillrank _itemowner_2 _itemownerimage_2 _rowindex))
      (break))))

(fn `FindClosestEnemy`
  (locals (`Object Types` :type "Array of EObjectTypeQuery Enum") (NewLocalVar :type "Array of Actor Object Reference"))
  (bind _controlledplayercharacter (`self.ControlledPlayerCharacter`))
  (bind _outactors (`KismetSystemLibrary.SphereOverlapActors` (`self.K2_GetActorLocation` (`self.ControlledPlayerCharacter`)) 512.0 (`local.Object Types`) "/Script/WutheringWaves.EnemyCharacter"))
  (bind _output_get (set `local.NewLocalVar` _outactors))
  (if (`KismetArrayLibrary.Array_IsEmpty` _output_get)
    (set `self.ClosestEnemy` null)
    (else
      ;[1 1 1] 조우 시에는 대쉬없어도 타겟 잡기
      (`/Engine/EditorBlueprintResources/StandardMacros.IsValid` (`self.ClosestEnemy`)
        (:`Is Valid`
          (`WWBlueprintFunctionLibrary.BP_HasTag` _controlledplayercharacter (struct :`TagName` "Player.Status.Dashing")
            (:`Yes`
              (if (> (`KismetMathLibrary.VSize2D` (`self.IsInputMove`)) 0.0)
                (set `self.ClosestEnemy` (`.ReturnValue` (`GameplayStatics.FindNearestActor` (`self.K2_GetActorLocation` _controlledplayercharacter) (`local.NewLocalVar`))))))))
        (:`Is Not Valid`
          (set `self.ClosestEnemy` (`.ReturnValue` (`GameplayStatics.FindNearestActor` (`self.K2_GetActorLocation` (`self.ControlledPlayerCharacter`)) (`local.NewLocalVar`)))))))))

(fn `UserConstructionScript`)