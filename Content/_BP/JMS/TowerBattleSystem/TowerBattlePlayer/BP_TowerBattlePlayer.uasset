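; Tower battle runner that plays a timed, three-wave encounter with looping battle music when the battle starts.
; A Wave macro runs async ExecuteWave on WavesToPlay at the actor's transform, each clear chaining the next wave.
; The level's BP_LevelTimer drives the HUD timer through the player controller's shared UI component.
; Timer expiry broadcasts battle failed; clearing the last wave broadcasts battle cleared and stops the timer.
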(event `self.ReceiveBeginPlay`)

(event `self.OnTowerBattleStart`
  (`GameplayStatics.PlaySound2D` "/Game/_BP/JMS/BGM/SC_BattleBGM_Loop.SC_BattleBGM_Loop" 1.0 1.0 0.0 null null)
  (bind _output_get (`self.FindTimerAndHUDUIComponent`))
  (`WWHUDSharedUIComponent.BroadcastHUDTimerEnabled` _output_get true)
  (add `WWLevelTimer.OnTimerUpdate` (`self.TimerActorOnCurrentLevel`) (delegate `OnTimerUpdate_Event`))
  (`WWLevelTimer.StartTimer` (`self.TimerActorOnCurrentLevel`) (`self.BattleTimeLimit`) 0.1)
  (add `WWLevelTimer.OnTimerEnd` (`self.TimerActorOnCurrentLevel`) (delegate `BattleFailedEvent`))
  (`self.Wave` 0
    (:`OnWaveClear`
      (`self.Wave` 1
        (:`OnWaveClear`
          (`self.Wave` 2
            (:`OnWaveClear`
              (`self.BroadcastOnBattleClearedDelegate`)
              (`WWLevelTimer.StopTimer` (`self.TimerActorOnCurrentLevel`)))))))))

(event `BattleFailedEvent`
  (`self.BroadcastOnBattleFailedDelegate`))

(event `OnTimerUpdate_Event`
  (params (NewTime :type "Float (single-precision)"))
  (`WWHUDSharedUIComponent.BroadcastHUDTimerUpdate` (`self.HUDUIComponentReference`) NewTime))

(fn `FindTimerAndHUDUIComponent`
  (returns (Output_Get :type "WWHUDSharedUIComponent Object Reference"))
  (bind _returnvalue (`GameplayStatics.GetActorOfClass` "/Game/_BP/JMS/TowerBattleSystem/LevelTimerActor/BP_LevelTimer.BP_LevelTimer_C"))
  (set `self.TimerActorOnCurrentLevel` _returnvalue)
  (bind _returnvalue_2 (message `WWHUDSharedUIInterface.GetHUDSharedUIComponent` (`GameplayStatics.GetPlayerController` 0)))
  (bind _output_get (set `self.HUDUIComponentReference` _returnvalue_2))
  (return _output_get))

(fn `UserConstructionScript`)