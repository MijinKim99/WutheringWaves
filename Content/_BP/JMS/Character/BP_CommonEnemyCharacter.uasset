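; BP_CommonEnemyCharacter is a common enemy character Blueprint that handles the visual death sequence and reports the death to its group.
; On OnEnemyDie it pauses mesh animation and disables capsule collision and gravity, then async-loads and attaches the supplied Niagara VFX.
; A timeline scaled by DissolveTime drives the DissolveAmount material parameter.
; When it finishes, the actor is hidden and moved far away rather than destroyed, and its owning WWEnemyGroup is notified via EnemyDead.
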(event `/Game/_BP/JMS/Character/BlueprintInterface/BPI_EnemyDeath.OnEnemyDie`
  (params (VFX :type "NiagaraSystem Soft Object Reference"))
  (`|ExecutionSequence`
    (:`then_0`
      (set `SkeletalMeshComponent.bPauseAnims` true (`self.Mesh`))
      (`PrimitiveComponent.SetCollisionEnabled` (`self.CapsuleComponent`) "NoCollision")
      (`PrimitiveComponent.SetEnableGravity` (`self.CapsuleComponent`) false))
    (:`then_1`
      (bind _object (`|LoadAsset` VFX)
        (:`Completed`
          (bind _asniagara_system (cast `NiagaraSystem` _object)
            (:`then`
              (`NiagaraFunctionLibrary.SpawnSystemAttached` _asniagara_system null "None" (0.0 0.0 0.0) (struct) "KeepRelativeOffset"))
            (:`CastFailed`
              _))
          (`TimelineComponent.SetPlayRate` (`self.DissolveTimeLine`) (/ 1.0 (`self.DissolveTime`)))
          (bind (_direction _newtrack_0) (`Timeline|DissolveTimeLine` :!via `PlayFromStart`)
            (:`Update`
              (`MeshComponent.SetScalarParameterValueOnMaterials` (`self.Mesh`) "DissolveAmount" _newtrack_0))
            (:`Finished`
              (`self.SetActorHiddenInGame` true)
              (`self.K2_SetActorLocation` (100000.0 100000.0 100000.0))
              (bind _aswwenemy_group (cast `WWEnemyGroup` (`self.GetOwner`)))
              (`WWEnemyGroup.EnemyDead` _aswwenemy_group self))))))))

(fn `UserConstructionScript`)