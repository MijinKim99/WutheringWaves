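; Player controller, apparently for widget testing, that captures player input and holds the weapon inventory.
; Enhanced Input actions store the move vector and briefly pulse dash, jump and light-attack flags, while possession changes forward BP_PlayerCharacter to custom calls.
; BeginPlay fills InventoryWeapon from DT_Inventory_Weapon.
; ChangeWeapon clears the first entry matching the previous weapon's owner, then assigns that owner and image to the new weapon at the given index.
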(event `EnhancedInput|/Game/_BP/YHG/Inputs/Actions/IA_Move`
  (params (ActionValue :type "Vector2D Structure") (ElapsedSeconds :type "Float (double-precision)") (TriggeredSeconds :type "Float (double-precision)") (InputAction :type "InputAction Object Reference" :default "/Game/_BP/YHG/Inputs/Actions/IA_Move.IA_Move"))
  (:`Triggered`
    (set `self.IsInputMove` ActionValue))
  (:`Completed`
    (set `self.IsInputMove` (0.0 0.0))))

(event `EnhancedInput|/Game/_BP/YHG/Inputs/Actions/IA_Dash`
  (params (ActionValue :type Boolean) (ElapsedSeconds :type "Float (double-precision)") (TriggeredSeconds :type "Float (double-precision)") (InputAction :type "InputAction Object Reference" :default "/Game/_BP/YHG/Inputs/Actions/IA_Dash.IA_Dash"))
  (:`Started`
    (set `self.bIsInputDash` true)
    (`KismetSystemLibrary.Delay` 0.05)
    (set `self.bIsInputDash` false)))

(event `EnhancedInput|/Game/_BP/YHG/Inputs/Actions/IA_Jump`
  (params (ActionValue :type Boolean) (ElapsedSeconds :type "Float (double-precision)") (TriggeredSeconds :type "Float (double-precision)") (InputAction :type "InputAction Object Reference" :default "/Game/_BP/YHG/Inputs/Actions/IA_Jump.IA_Jump"))
  (:`Started`
    (set `self.bIsInputJump` true)
    (`KismetSystemLibrary.Delay` 0.05)
    (set `self.bIsInputJump` false)))

(event `EnhancedInput|/Game/_BP/YHG/Inputs/Actions/IA_LightAttack`
  (params (ActionValue :type Boolean) (ElapsedSeconds :type "Float (double-precision)") (TriggeredSeconds :type "Float (double-precision)") (InputAction :type "InputAction Object Reference" :default "/Game/_BP/YHG/Inputs/Actions/IA_LightAttack.IA_LightAttack"))
  (:`Started`
    (set `self.bIsInputLightAttack` true)
    (`KismetSystemLibrary.Delay` 0.05)
    (set `self.bIsInputLightAttack` false)))

(event `self.ReceiveTick`
  (params (DeltaSeconds :type "Float (single-precision)")))

(event `self.ReceivePossess`
  (params (PossessedPawn :type "Pawn Object Reference"))
  (bind _asbp_player_character (cast `/Game/_BP/YHG/Characters/BP_PlayerCharacter` PossessedPawn))
  (`self.OnPossessPawnCustom` _asbp_player_character))

(event `self.ReceiveUnPossess`
  (params (UnpossessedPawn :type "Pawn Object Reference"))
  (bind _asbp_player_character (cast `/Game/_BP/YHG/Characters/BP_PlayerCharacter` UnpossessedPawn))
  (`self.OnUnPossessPawnCustom` _asbp_player_character))

(event `self.ReceiveBeginPlay`
  (`KismetArrayLibrary.Array_Clear` (`self.Inventory_Weapon`))
  (bind _outrownames (`DataTableFunctionLibrary.GetDataTableRowNames` "/Game/_BP/KMJ/DataTable/Weapons/DT_Inventory_Weapon.DT_Inventory_Weapon"))
  (for _array_element _outrownames
    (bind _returnvalue (`|GetDataTableRow` "/Game/_BP/KMJ/DataTable/Weapons/DT_Inventory_Weapon.DT_Inventory_Weapon" _array_element)
      (:`then`
        (`KismetArrayLibrary.Array_Add` (`self.Inventory_Weapon`) _returnvalue)))))

(event `/Game/_BP/KMJ/Interface/BPI_ChangeWeapon.ChangeWeapon`
  (params (PreviousWeapon :type "Inventory_Weapon Structure") (NewWeapon :type "Inventory_Weapon Structure") (Index :type Integer))
  (`self.ChangeEquippedWeapon` PreviousWeapon NewWeapon Index))

(fn `ChangeEquippedWeapon`
  (params (PreviousWeapon :type "Inventory_Weapon Structure") (NewWeapon :type "Inventory_Weapon Structure") (Index :type Integer))
  (bind (_weaponcurrentlevel _weaponcurrentrank _skillrank _itemowner _itemownerimage _rowindex) (break `Inventory_Weapon` NewWeapon))
  (bind (_weaponcurrentlevel_2 _weaponcurrentrank_2 _skillrank_2 _itemowner_2 _itemownerimage_2) (break `Inventory_Weapon` PreviousWeapon))
  (for (_array_element _array_index) (`self.Inventory_Weapon`)
    (bind (_weaponcurrentlevel_3 _weaponcurrentrank_3 _skillrank_3 _itemowner_3 _itemownerimage_3 _rowindex_2) (break `Inventory_Weapon` _array_element))
    (if (`|EnumEquality` _itemowner_3 _itemowner_2)
      (`KismetArrayLibrary.Array_Set` (`self.Inventory_Weapon`) _array_index (make `Inventory_Weapon` _weaponcurrentlevel_3 _weaponcurrentrank_3 _skillrank_3 "None" _itemownerimage_3 _rowindex_2))
      (break)))
  (for (_ _array_index_2) (`self.Inventory_Weapon`)
    (if (== Index _array_index_2)
      (`KismetArrayLibrary.Array_Set` (`self.Inventory_Weapon`) _array_index_2 (make `Inventory_Weapon` _weaponcurrentlevel _weaponcurrentrank _skillrank _itemowner_2 _itemownerimage_2 _rowindex))
      (break))))

(fn `IsWeaponDataEqual`
  (params (WeaponData1 :type "Inventory_Weapon Structure") (WeaponData2 :type "Inventory_Weapon Structure"))
  (returns (NewParam :type Boolean))
  (bind (_weaponcurrentlevel _weaponcurrentrank _skillrank _itemowner _itemownerimage _rowindex) (break `Inventory_Weapon` WeaponData1))
  (bind (_weaponcurrentlevel_2 _weaponcurrentrank_2 _skillrank_2 _itemowner_2 _itemownerimage_2 _rowindex_2) (break `Inventory_Weapon` WeaponData2))
  (return (and (== _weaponcurrentlevel _weaponcurrentlevel_2) (== _weaponcurrentrank _weaponcurrentrank_2) (== _skillrank _skillrank_2) (`|EnumEquality` _itemowner) (== _itemownerimage _itemownerimage_2) (`KismetStringLibrary.EqualEqual_StrStr` _rowindex _rowindex_2))))

(fn `UserConstructionScript`)