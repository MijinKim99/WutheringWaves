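; Player controller for a widget test with a three-character party (Rover, Chixia, Verina), handling input, character switching, HUD and menus.
; Move input is stored, dash, jump and attack briefly pulse flags, and character keys possess another member unless on cooldown, updating party icons and minimap capture.
; BeginPlay builds the HUD and loads the weapon inventory from a DataTable, which ChangeWeapon edits to move weapon ownership.
; C and B open character and inventory screens and pause the game.
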(event `EnhancedInput|/Game/_BP/YHG/Inputs/Actions/IA_Move`
  (params (ActionValue :type "Vector2D Structure") (ElapsedSeconds :type "Float (double-precision)") (TriggeredSeconds :type "Float (double-precision)") (InputAction :type "InputAction Object Reference" :default "/Game/_BP/YHG/Inputs/Actions/IA_Move.IA_Move"))
  (:`Triggered`
    (set `self.IsInputMove` ActionValue))
  (:`Completed`
    (set `self.IsInputMove` (0.0 0.0))))

(event `EnhancedInput|/Game/_BP/YHG/Inputs/Actions/IA_Dash`
  (params (ActionValue :type Boolean) (ElapsedSeconds :type "Float (double-precision)") (TriggeredSeconds :type "Float (double-precision)") (InputAction :type "InputAction Object Reference" :default "/Game/_BP/YHG/Inputs/Actions/IA_Dash.IA_Dash"))
  (:`Started`
    (set `self.bIsInputDash` true)
    (`KismetSystemLibrary.Delay` 0.05)
    (set `self.bIsInputDash` false)))

(event `EnhancedInput|/Game/_BP/YHG/Inputs/Actions/IA_Jump`
  (params (ActionValue :type Boolean) (ElapsedSeconds :type "Float (double-precision)") (TriggeredSeconds :type "Float (double-precision)") (InputAction :type "InputAction Object Reference" :default "/Game/_BP/YHG/Inputs/Actions/IA_Jump.IA_Jump"))
  (:`Started`
    (set `self.bIsInputJump` true)
    (`KismetSystemLibrary.Delay` 0.05)
    (set `self.bIsInputJump` false)))

(event `EnhancedInput|/Game/_BP/YHG/Inputs/Actions/IA_LightAttack`
  (params (ActionValue :type Boolean) (ElapsedSeconds :type "Float (double-precision)") (TriggeredSeconds :type "Float (double-precision)") (InputAction :type "InputAction Object Reference" :default "/Game/_BP/YHG/Inputs/Actions/IA_LightAttack.IA_LightAttack"))
  (:`Started`
    (set `self.bIsInputLightAttack` true)
    (`KismetSystemLibrary.Delay` 0.05)
    (set `self.bIsInputLightAttack` false)))

(event `EnhancedInput|/Game/_BP/YHG/Inputs/Actions/IA_Character1`
  (params (ActionValue :type Boolean) (ElapsedSeconds :type "Float (double-precision)") (TriggeredSeconds :type "Float (double-precision)") (InputAction :type "InputAction Object Reference" :default "/Game/_BP/YHG/Inputs/Actions/IA_Character1.IA_Character1"))
  (bind _widget_playerhud (`self.Widget_PlayerHUD`))
  (bind _wbp_party_icons (`/Game/_BP/KMJ/Widget/HUD/WBP_PlayerHUD.WBP_Party_Icons` _widget_playerhud))
  (:`Started`
    (`/Engine/EditorBlueprintResources/StandardMacros.IsValid` _widget_playerhud
      (:`Is Valid`
        (if (not (`/Game/_BP/KMJ/Widget/HUD/Assets/PartyIcon/WBP_HUD_PartyButton.IsCoolTime` (`/Game/_BP/KMJ/Widget/HUD/Assets/WBP_Party_Icons_HUD.WBP_HUD_PartyButton_Rover` _wbp_party_icons)))
          (bind _returnvalue (`GameplayStatics.GetActorOfClass` "/Game/_BP/YHG/Characters/LightRover/BP_LightRoverCharacter.BP_LightRoverCharacter_C"))
          (`/Engine/EditorBlueprintResources/StandardMacros.IsValid` _returnvalue
            (:`Is Valid`
              (if (!= _returnvalue (`self.ControlledPlayerCharacter`))
                (`self.Possess` _returnvalue)
                (`SkeletalMeshComponent.SetAnimInstanceClass` (`Character.Mesh` _returnvalue) "/Game/_BP/YHG/Characters/LightRover/Animation/ABP_LightRoverAnim.ABP_LightRoverAnim_C")
                (`WWBlueprintFunctionLibrary.AddTagToActor` (`self.PlayerState`))
                (`/Game/_BP/KMJ/Widget/HUD/Assets/WBP_Party_Icons_HUD.CharacterChange_Event` _wbp_party_icons "Rover")
                (`self.ChangeMiniMapCamera` true)))))))))

(event `EnhancedInput|/Game/_BP/YHG/Inputs/Actions/IA_Character2`
  (params (ActionValue :type Boolean) (ElapsedSeconds :type "Float (double-precision)") (TriggeredSeconds :type "Float (double-precision)") (InputAction :type "InputAction Object Reference" :default "/Game/_BP/YHG/Inputs/Actions/IA_Character2.IA_Character2"))
  (bind _widget_playerhud (`self.Widget_PlayerHUD`))
  (bind _wbp_party_icons (`/Game/_BP/KMJ/Widget/HUD/WBP_PlayerHUD.WBP_Party_Icons` _widget_playerhud))
  (:`Started`
    (`/Engine/EditorBlueprintResources/StandardMacros.IsValid` _widget_playerhud
      (:`Is Valid`
        (if (not (`/Game/_BP/KMJ/Widget/HUD/Assets/PartyIcon/WBP_HUD_PartyButton.IsCoolTime` (`/Game/_BP/KMJ/Widget/HUD/Assets/WBP_Party_Icons_HUD.WBP_HUD_PartyButton_Chixia` _wbp_party_icons)))
          (bind _returnvalue (`GameplayStatics.GetActorOfClass` "/Game/_BP/YHG/Characters/Chixia/BP_ChixiaCharacter.BP_ChixiaCharacter_C"))
          (`/Engine/EditorBlueprintResources/StandardMacros.IsValid` _returnvalue
            (:`Is Valid`
              (if (!= _returnvalue (`self.ControlledPlayerCharacter`))
                (`self.Possess` _returnvalue)
                (`SkeletalMeshComponent.SetAnimInstanceClass` (`Character.Mesh` _returnvalue) "/Game/_BP/YHG/Characters/Chixia/Animation/ABP_ChixiaAnim.ABP_ChixiaAnim_C")
                (`/Game/_BP/KMJ/Widget/HUD/Assets/WBP_Party_Icons_HUD.CharacterChange_Event` _wbp_party_icons "Chixia")
                (`self.ChangeMiniMapCamera` false true)))))))))

(event `EnhancedInput|/Game/_BP/YHG/Inputs/Actions/IA_Character3`
  (params (ActionValue :type Boolean) (ElapsedSeconds :type "Float (double-precision)") (TriggeredSeconds :type "Float (double-precision)") (InputAction :type "InputAction Object Reference" :default "/Game/_BP/YHG/Inputs/Actions/IA_Character3.IA_Character3"))
  (bind _widget_playerhud (`self.Widget_PlayerHUD`))
  (bind _wbp_party_icons (`/Game/_BP/KMJ/Widget/HUD/WBP_PlayerHUD.WBP_Party_Icons` _widget_playerhud))
  (:`Started`
    (`/Engine/EditorBlueprintResources/StandardMacros.IsValid` _widget_playerhud
      (:`Is Valid`
        (if (not (`/Game/_BP/KMJ/Widget/HUD/Assets/PartyIcon/WBP_HUD_PartyButton.IsCoolTime` (`/Game/_BP/KMJ/Widget/HUD/Assets/WBP_Party_Icons_HUD.WBP_HUD_PartyButton_Verina` _wbp_party_icons)))
          (bind _returnvalue (`GameplayStatics.GetActorOfClass` "/Game/_BP/YHG/Characters/Verina/BP_VerinaCharacter.BP_VerinaCharacter_C"))
          (`/Engine/EditorBlueprintResources/StandardMacros.IsValid` _returnvalue
            (:`Is Valid`
              (if (!= _returnvalue (`self.ControlledPlayerCharacter`))
                (`self.Possess` _returnvalue)
                (`SkeletalMeshComponent.SetAnimInstanceClass` (`Character.Mesh` _returnvalue) "/Game/_BP/YHG/Characters/Verina/Animation/ABP_VerinaAnim.ABP_VerinaAnim_C")
                (`/Game/_BP/KMJ/Widget/HUD/Assets/WBP_Party_Icons_HUD.CharacterChange_Event` _wbp_party_icons "Verina")
                (`self.ChangeMiniMapCamera` false false true)))))))))

(event `self.ReceivePossess`
  (params (PossessedPawn :type "Pawn Object Reference")))

(event `self.ReceiveUnPossess`
  (params (UnpossessedPawn :type "Pawn Object Reference")))

(event `self.ReceiveBeginPlay`
  (bind _widget_playerhud (`self.Widget_PlayerHUD`))
  (bind _character_rover (`self.Character_Rover`))
  (`KismetArrayLibrary.Array_Clear` (`self.Inventory_Weapon`))
  (bind _outrownames (`DataTableFunctionLibrary.GetDataTableRowNames` "/Game/_BP/KMJ/DataTable/Weapons/DT_Inventory_Weapon.DT_Inventory_Weapon"))
  (for _array_element _outrownames
    (bind _returnvalue (`|GetDataTableRow` "/Game/_BP/KMJ/DataTable/Weapons/DT_Inventory_Weapon.DT_Inventory_Weapon" _array_element)
      (:`then`
        (`KismetArrayLibrary.Array_Add` (`self.Inventory_Weapon`) _returnvalue))))
  (bind _returnvalue_2 (`|CreateWidget` "/Game/_BP/KMJ/Widget/HUD/WBP_PlayerHUD.WBP_PlayerHUD_C"))
  (bind _output_get (set `self.Widget_PlayerHUD` _returnvalue_2))
  (`UserWidget.AddToViewport` _output_get 0)
  (bind _returnvalue_3 (`GameplayStatics.GetActorOfClass` "/Game/_BP/YHG/Characters/LightRover/BP_LightRoverCharacter.BP_LightRoverCharacter_C"))
  (set `self.Character_Rover` _returnvalue_3)
  (bind _returnvalue_4 (`GameplayStatics.GetActorOfClass` "/Game/_BP/YHG/Characters/Chixia/BP_ChixiaCharacter.BP_ChixiaCharacter_C"))
  (set `self.Character_Chixia` _returnvalue_4)
  (bind _returnvalue_5 (`GameplayStatics.GetActorOfClass` "/Game/_BP/YHG/Characters/Verina/BP_VerinaCharacter.BP_VerinaCharacter_C"))
  (set `self.Character_Verina` _returnvalue_5)
  (`self.ChangeMiniMapCamera` true)
  (`/Game/_BP/KMJ/Widget/HUD/Assets/WBP_Party_Icons_HUD.LinkCharacterHPBarToCharacter` (`/Game/_BP/KMJ/Widget/HUD/WBP_PlayerHUD.WBP_Party_Icons` _widget_playerhud) _character_rover (`self.Character_Chixia`) (`self.Character_Verina`))
  (`/Game/_BP/KMJ/Widget/HUD/WBP_PlayerHUD.LinkPawnHP` _widget_playerhud _character_rover))

(event `/Game/_BP/KMJ/Interface/BPI_ChangeWeapon.ChangeWeapon`
  (params (PreviousWeapon :type "Inventory_Weapon Structure") (NewWeapon :type "Inventory_Weapon Structure") (Index :type Integer))
  (`self.ChangeEquippedWeapon` PreviousWeapon NewWeapon Index))

(event `Key|C`
  (params (Key :type "Key Structure"))
  (:`Pressed`
    (`/Game/_BP/KMJ/Widget/CharacterSetting/BP_CharSettingUIComponent.CreateWidget_CharSetting` (`self.BP_CharSettingUIComponent`))
    (`Widget.SetVisibility` (`self.Widget_PlayerHUD`) "Hidden")
    (`GameplayStatics.SetGamePaused` true)))

(event `Key|B`
  (params (Key :type "Key Structure"))
  (:`Pressed`
    (`/Game/_BP/KMJ/Widget/CharacterSetting/BP_CharSettingUIComponent.CreateWidget_Inventory` (`self.BP_CharSettingUIComponent`))
    (`GameplayStatics.SetGamePaused` true)))

(fn `ChangeEquippedWeapon`
  (params (PreviousWeapon :type "Inventory_Weapon Structure") (NewWeapon :type "Inventory_Weapon Structure") (Index :type Integer))
  (bind (_weaponcurrentlevel _weaponcurrentrank _skillrank _itemowner _itemownerimage _rowindex) (break `Inventory_Weapon` NewWeapon))
  (bind (_weaponcurrentlevel_2 _weaponcurrentrank_2 _skillrank_2 _itemowner_2 _itemownerimage_2) (break `Inventory_Weapon` PreviousWeapon))
  ;[0.2969 0.2969 0.2969] 무기 장착 해제
  (for (_array_element _array_index) (`self.Inventory_Weapon`)
    (bind (_weaponcurrentlevel_3 _weaponcurrentrank_3 _skillrank_3 _itemowner_3 _itemownerimage_3 _rowindex_2) (break `Inventory_Weapon` _array_element))
    (if (`|EnumEquality` _itemowner_3 _itemowner_2)
      (`KismetArrayLibrary.Array_Set` (`self.Inventory_Weapon`) _array_index (make `Inventory_Weapon` _weaponcurrentlevel_3 _weaponcurrentrank_3 _skillrank_3 "None" _itemownerimage_3 _rowindex_2))
      (break)))
  ;[0.2708 0.2708 0.2708] 무기 새로 장착
  (for (_ _array_index_2) (`self.Inventory_Weapon`)
    (if (== Index _array_index_2)
      (`KismetArrayLibrary.Array_Set` (`self.Inventory_Weapon`) _array_index_2 (make `Inventory_Weapon` _weaponcurrentlevel _weaponcurrentrank _skillrank _itemowner_2 _itemownerimage_2 _rowindex))
      (break))))

(fn `ChangeMiniMapCamera`
  (params (Rover :type Boolean) (Chixia :type Boolean) (Verina :type Boolean))
  (`SceneComponent.SetVisibility` (`/Game/_BP/YHG/Characters/LightRover/BP_LightRoverCharacter.SceneCaptureComponent2D` (`self.Character_Rover`)) Rover true)
  (`SceneComponent.SetVisibility` (`/Game/_BP/YHG/Characters/Chixia/BP_ChixiaCharacter.SceneCaptureComponent2D` (`self.Character_Chixia`)) Chixia true)
  (`SceneComponent.SetVisibility` (`/Game/_BP/YHG/Characters/Verina/BP_VerinaCharacter.SceneCaptureComponent2D` (`self.Character_Verina`)) Verina true))

(fn `IsWeaponDataEqual`
  (params (WeaponData1 :type "Inventory_Weapon Structure") (WeaponData2 :type "Inventory_Weapon Structure"))
  (returns (NewParam :type Boolean))
  (bind (_weaponcurrentlevel _weaponcurrentrank _skillrank _itemowner _itemownerimage _rowindex) (break `Inventory_Weapon` WeaponData1))
  (bind (_weaponcurrentlevel_2 _weaponcurrentrank_2 _skillrank_2 _itemowner_2 _itemownerimage_2 _rowindex_2) (break `Inventory_Weapon` WeaponData2))
  (return (and (== _weaponcurrentlevel _weaponcurrentlevel_2) (== _weaponcurrentrank _weaponcurrentrank_2) (== _skillrank _skillrank_2) (`|EnumEquality` _itemowner) (== _itemownerimage _itemownerimage_2) (`KismetStringLibrary.EqualEqual_StrStr` _rowindex _rowindex_2))))

(fn `UserConstructionScript`)