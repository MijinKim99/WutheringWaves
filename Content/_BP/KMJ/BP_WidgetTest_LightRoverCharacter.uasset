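; BP_WidgetTest_LightRoverCharacter is a test character for opening the character setting and inventory widgets.
; On BeginPlay it hides the scabbard and sword and disables sword collision.
; The C and B keys call BPCharSettingUIComponent to create the character setting or inventory widget, then pause the game.
; An unconnected branch would switch the view to BP_SceneCapture2D_ForUI before opening character settings.
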(event `self.ReceiveBeginPlay`
  (`|ExecutionSequence`
    (:`then_0`
      (`SceneComponent.SetVisibility` (`self.Scabbard`) false false)
      (`SceneComponent.SetVisibility` (`self.Sword`) false false))
    (:`then_1`
      (`PrimitiveComponent.SetCollisionEnabled` (`self.Sword`) "NoCollision"))))

(event `Key|C`
  (params (Key :type "Key Structure"))
  (:`Pressed`
    (`/Game/_BP/KMJ/Widget/CharacterSetting/BP_CharSettingUIComponent.CreateWidget_CharSetting` (`self.BP_CharSettingUIComponent`))
    (`GameplayStatics.SetGamePaused` true)))

(event `Key|B`
  (params (Key :type "Key Structure"))
  (:`Pressed`
    (`/Game/_BP/KMJ/Widget/CharacterSetting/BP_CharSettingUIComponent.CreateWidget_Inventory` (`self.BP_CharSettingUIComponent`))
    (`GameplayStatics.SetGamePaused` true)))

(fn `UserConstructionScript`)