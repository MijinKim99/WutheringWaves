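; Gameplay Ability for the player's air dash, usable only while airborne and while CanAirDash is set.
; On activation it sets sprint mode, clears attack mode and consumes the air dash.
; With move input, it snaps the character to face the camera-relative input direction and plays the forward dash montage; without input, it plays the back dash montage.
; The ability ends when the montage finishes, blends out or is interrupted, or immediately if the dash is unavailable.
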(event `self.K2_ActivateAbility`
  (bind _returnvalue (`self.GetPlayerCharacterFromActorInfo`))
  (if (and (not (`PlayerCharacter.bIsGrounded` _returnvalue)) (`PlayerCharacter.bCanAirDash` _returnvalue))
    (`self.ChangeState`)
    (if (`KismetMathLibrary.NotEqualExactly_Vector2DVector2D` (`WWPlayerController.IsInputMove` (`self.GetPlayerControllerFromActorInfo`)))
      (`self.RotateMoveDirection`)
      (`AbilityTask_PlayMontageAndWait.CreatePlayMontageAndWaitProxy` "None" (`PlayerCharacter.FAirDash` (`self.GetPlayerCharacterFromActorInfo`))
        (:`OnCompleted`
          _)
        (:`OnBlendOut`
          _)
        (:`OnInterrupted`
          _)
        (:`OnCancelled`
          _))
      (`self.K2_EndAbility`)
      (else
        (`AbilityTask_PlayMontageAndWait.CreatePlayMontageAndWaitProxy` "None" (`PlayerCharacter.BAirDash` (`self.GetPlayerCharacterFromActorInfo`))
          (:`OnCompleted`
            _)
          (:`OnBlendOut`
            _)
          (:`OnInterrupted`
            _)
          (:`OnCancelled`
            _))
        (`self.K2_EndAbility`)))
    (else
      (`self.K2_EndAbility`))))

(fn `ChangeState`
  (bind _returnvalue (`self.GetPlayerCharacterFromActorInfo`))
  (set `PlayerCharacter.bSprintMode` true _returnvalue)
  (set `PlayerCharacter.bAttackMode` false _returnvalue)
  (set `PlayerCharacter.bCanAirDash` false _returnvalue))

(fn `RotateMoveDirection`
  (bind _followcamera (`PlayerCharacter.FollowCamera` (`self.GetPlayerCharacterFromActorInfo`)))
  (bind (_returnvalue_x _returnvalue_y) (`KismetMathLibrary.BreakVector` (`SceneComponent.GetRightVector` _followcamera)))
  (bind (_x _y) (`KismetMathLibrary.BreakVector2D` (`WWPlayerController.IsInputMove` (`self.GetPlayerControllerFromActorInfo`))))
  (bind (_returnvalue_x_2 _returnvalue_y_2) (`KismetMathLibrary.BreakVector` (`SceneComponent.GetForwardVector` _followcamera)))
  (bind _returnvalue (+ (* (`KismetMathLibrary.Normal` (`KismetMathLibrary.MakeVector` _returnvalue_x _returnvalue_y)) _x) (* (`KismetMathLibrary.Normal` (`KismetMathLibrary.MakeVector` _returnvalue_x_2 _returnvalue_y_2)) _y)))
  (if (`KismetMathLibrary.NotEqualExactly_VectorVector` _returnvalue)
    (`Actor.K2_SetActorRotation` (`self.GetPlayerCharacterFromActorInfo`) (`KismetMathLibrary.MakeRotFromX` _returnvalue) true)))