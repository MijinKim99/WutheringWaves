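; Gameplay ability for the player's ground dash, limited to a grounded character with fewer than two dashes counted.
; On activation it increments the dash count and clears attack mode.
; With move input it snaps the character to the camera-relative input direction, enables sprint mode and plays the forward dash montage; without input it plays a fixed backward-move montage.
; The ability ends when the montage finishes, blends out or is interrupted.
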(event `self.K2_ActivateAbility`
  (bind _returnvalue (`self.GetPlayerCharacterFromActorInfo`))
  (bind _returnvalue_2 (`self.GetPlayerCharacterFromActorInfo`))
  (if (and (`PlayerCharacter.bIsGrounded` _returnvalue_2) (< (`PlayerCharacter.DashCount` _returnvalue_2) 2))
    (set `PlayerCharacter.DashCount` (+ (`PlayerCharacter.DashCount` _returnvalue) 1) _returnvalue)
    (`self.ChangeState`)
    (if (`KismetMathLibrary.NotEqualExactly_Vector2DVector2D` (`WWPlayerController.IsInputMove` (`self.GetPlayerControllerFromActorInfo`)))
      (`self.RotateMoveDirection`)
      (set `PlayerCharacter.bSprintMode` true (`self.GetPlayerCharacterFromActorInfo`))
      (`AbilityTask_PlayMontageAndWait.CreatePlayMontageAndWaitProxy` "None" (`PlayerCharacter.FGroundDash` (`self.GetPlayerCharacterFromActorInfo`))
        (:`OnCompleted`
          _)
        (:`OnBlendOut`
          _)
        (:`OnInterrupted`
          _)
        (:`OnCancelled`
          _))
      (`self.K2_EndAbility`)
      (else
        (`AbilityTask_PlayMontageAndWait.CreatePlayMontageAndWaitProxy` "None" "/Game/_BP/YHG/Characters/LightRover/Animation/UseAnimation/BasicAnim/Dash/AM_MaleMBaseAnim_R2T1PlayerMaleMd10011_Lod4_Move_B_Edited.AM_MaleMBaseAnim_R2T1PlayerMaleMd10011_Lod4_Move_B_Edited"
          (:`OnCompleted`
            _)
          (:`OnBlendOut`
            _)
          (:`OnInterrupted`
            _)
          (:`OnCancelled`
            _))
        (`self.K2_EndAbility`)))
    (else
      (`self.K2_EndAbility`))))

(event `self.K2_OnEndAbility`
  (params (bWasCancelled :type Boolean)))

(fn `ChangeState`
  (set `PlayerCharacter.bAttackMode` false (`self.GetPlayerCharacterFromActorInfo`)))

(fn `RotateMoveDirection`
  (bind _followcamera (`PlayerCharacter.FollowCamera` (`self.GetPlayerCharacterFromActorInfo`)))
  (bind (_returnvalue_x _returnvalue_y) (`KismetMathLibrary.BreakVector` (`SceneComponent.GetRightVector` _followcamera)))
  (bind (_x _y) (`KismetMathLibrary.BreakVector2D` (`WWPlayerController.IsInputMove` (`self.GetPlayerControllerFromActorInfo`))))
  (bind (_returnvalue_x_2 _returnvalue_y_2) (`KismetMathLibrary.BreakVector` (`SceneComponent.GetForwardVector` _followcamera)))
  (bind _returnvalue (+ (* (`KismetMathLibrary.Normal` (`KismetMathLibrary.MakeVector` _returnvalue_x _returnvalue_y)) _x) (* (`KismetMathLibrary.Normal` (`KismetMathLibrary.MakeVector` _returnvalue_x_2 _returnvalue_y_2)) _y)))
  (if (`KismetMathLibrary.NotEqualExactly_VectorVector` _returnvalue)
    (`Actor.K2_SetActorRotation` (`self.GetPlayerCharacterFromActorInfo`) (`KismetMathLibrary.MakeRotFromX` _returnvalue) true)))