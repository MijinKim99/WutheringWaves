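; Gameplay ability for Verina's aerial combo attack, which advances her air combo count and plays the matching attack montage.
; On a HitEnemy gameplay event, it shows her Rectifier weapon and fires a pooled box projectile from her spine socket.
; The projectile applies light, stagger and parry damage effects with a small hit react, targeting the controller's closest enemy when valid.
; The ability ends when the montage completes, blends out or is interrupted or cancelled.
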(event `self.K2_ActivateAbility`
  (bind _returnvalue (`self.GetPlayerCharacterFromActorInfo`))
  (`self.K2_CommitAbilityCost` false)
  (bind _asbp_verina_character (cast `/Game/_BP/YHG/Characters/Verina/BP_VerinaCharacter` (`self.GetPlayerCharacterFromActorInfo`)))
  (bind _verinaaircombocount (`/Game/_BP/YHG/Characters/Verina/BP_VerinaCharacter.VerinaAirComboCount` _asbp_verina_character))
  (set `/Game/_BP/YHG/Characters/Verina/BP_VerinaCharacter.VerinaAirComboCount` (+ _verinaaircombocount 1) _asbp_verina_character)
  (`AbilityTask_PlayMontageAndWait.CreatePlayMontageAndWaitProxy` "None" (`BlueprintMapLibrary.Map_Find` (`self.AttackMontageMap`) _verinaaircombocount)
    (:`then`
      (`|ExecutionSequence`
        (:`then_1`
          (set `PlayerCharacter.bAttackMode` true _returnvalue)
          (set `PlayerCharacter.bSprintMode` false _returnvalue))
        (:`then_2`
          (`AbilityTask_WaitGameplayEvent.WaitGameplayEvent` (struct :`TagName` "Player.Event.HitEnemy") null
            (:`EventReceived`
              (`self.AirAttackDamage`)
              (`self.VisibleWeapon`))))))
    (:`OnCompleted`
      (`self.K2_EndAbility` :!label _label))
    (:`OnBlendOut`
      (goto _label))
    (:`OnInterrupted`
      (goto _label))
    (:`OnCancelled`
      (goto _label))))

(event `self.K2_OnEndAbility`
  (params (bWasCancelled :type Boolean)))

(fn `AirAttackDamage`
  (bind _array (`|MakeArray` (`self.MakePlayerDamageGameplayEffectSpecHandle` "/Game/_BP/JMS/Character/AbilitySystem/GE/GE_Damaged_Enemy.GE_Damaged_Enemy_C" 5.0 (struct :`TagName` "Shared.SetByCaller.Damage.Light")) (`self.MakePlayerDamageGameplayEffectSpecHandle` "/Game/_BP/JMS/Character/AbilitySystem/GE/GE_Damaged_Enemy.GE_Damaged_Enemy_C" 10.0 (struct :`TagName` "Shared.SetByCaller.Damage.Stagger")) (`self.MakePlayerDamageGameplayEffectSpecHandle` "/Game/_BP/JMS/Character/AbilitySystem/GE/GE_Damaged_Enemy.GE_Damaged_Enemy_C" 7.5 (struct :`TagName` "Shared.SetByCaller.Damage.Parry"))))
  (bind _asbp_verina_character (cast `/Game/_BP/YHG/Characters/Verina/BP_VerinaCharacter` (`self.GetPlayerCharacterFromActorInfo`)))
  (bind _returnvalue (`WWObjectPoolComponent.SpawnPooledObject` (`/Game/_BP/YHG/Characters/Verina/BP_VerinaCharacter.VerinaBoxProjectileCollision` _asbp_verina_character) _asbp_verina_character))
  (bind _asbp_verina_box_projectile_collision (cast `/Game/_BP/YHG/Characters/Verina/AttackCollisionBP/BP_VerinaBoxProjectileCollision` _returnvalue))
  (bind _asbp_wwplayer_controller (cast `/Game/_BP/YHG/PlayerControllers/BP_WWPlayerController` (`self.GetPlayerControllerFromActorInfo`)))
  (bind _closestenemy (`/Game/_BP/YHG/PlayerControllers/BP_WWPlayerController.ClosestEnemy` _asbp_wwplayer_controller))
  (`/Engine/EditorBlueprintResources/StandardMacros.IsValid` _closestenemy
    (:`Is Valid`
      (bind _mesh (`Character.Mesh` _asbp_verina_character))
      (`AttackCollisionBoxProjectile.InitializeAttachedProjectileAndShootMultipleEffects` :`self` _asbp_verina_box_projectile_collision :`BoxExtent` (8.0 8.0 8.0) :`InstigatorMesh` _mesh :`AttachSocketName` "Bip001Spine2" :`InGameplayEffectSpecHandles` _array :`TargetLocation` (`Actor.K2_GetActorLocation` _closestenemy) :`ProjectileSpeed` 500000.0 :`InHitReactEventTag` (struct :`TagName` "Shared.Event.HitReact.Small") :`bShowCollisionInGame` true :`LineThickness` 5.0))
    (:`Is Not Valid`
      (`AttackCollisionBoxProjectile.InitializeAttachedProjectileAndShootMultipleEffects` :`self` _asbp_verina_box_projectile_collision :`BoxExtent` (8.0 8.0 8.0) :`InstigatorMesh` _mesh :`AttachSocketName` "Bip001Spine2" :`InGameplayEffectSpecHandles` _array :`ProjectileSpeed` 500000.0 :`InHitReactEventTag` (struct :`TagName` "Shared.Event.HitReact.Small") :`bShowCollisionInGame` true :`LineThickness` 5.0))))

(fn `HiddenWeapon`
  (bind _asbp_verina_character (cast `/Game/_BP/YHG/Characters/Verina/BP_VerinaCharacter` (`self.GetPlayerCharacterFromActorInfo`)))
  (`SceneComponent.SetVisibility` (`/Game/_BP/YHG/Characters/Verina/BP_VerinaCharacter.Rectifier` _asbp_verina_character) false false))

(fn `VisibleWeapon`
  (bind _asbp_verina_character (cast `/Game/_BP/YHG/Characters/Verina/BP_VerinaCharacter` (`self.GetPlayerCharacterFromActorInfo`)))
  (`SceneComponent.SetVisibility` (`/Game/_BP/YHG/Characters/Verina/BP_VerinaCharacter.Rectifier` _asbp_verina_character) true false))