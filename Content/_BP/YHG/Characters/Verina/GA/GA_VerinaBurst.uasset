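; Verina's burst gameplay ability, which plays an attack montage when she is grounded and ends otherwise.
; On start it commits cooldown and cost, then turns her toward camera-relative move input, overridden by the closest enemy if one is valid.
; Each received HitEnemy event spawns a pooled box collision around her that applies light, stagger and parry damage effects scaled from her attack, with a big hit reaction.
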(event `self.K2_ActivateAbility`
  (if (`PlayerCharacter.bIsGrounded` (`self.GetPlayerCharacterFromActorInfo`))
    (`AbilityTask_PlayMontageAndWait.CreatePlayMontageAndWaitProxy` "None" "/Game/_BP/YHG/Characters/Verina/Animation/UseAnimation/CharacterAnim/Burst/AM_VerinaAnim_R2T1JueyuanMd10011_Lod4_Burst01_Edited.AM_VerinaAnim_R2T1JueyuanMd10011_Lod4_Burst01_Edited"
      (:`then`
        (`AbilityTask_WaitGameplayEvent.WaitGameplayEvent` (struct :`TagName` "Player.Event.HitEnemy") null
          (:`then`
            (`self.K2_CommitAbilityCooldown` false)
            (`self.K2_CommitAbilityCost` false)
            (`self.RotateMoveDirection`)
            (`self.RotateEnemyDirection`))
          (:`EventReceived`
            (`self.GroundAttackDamage`))))
      (:`OnCompleted`
        (`self.K2_EndAbility` :!label _label))
      (:`OnBlendOut`
        (goto _label))
      (:`OnInterrupted`
        (goto _label))
      (:`OnCancelled`
        (goto _label)))
    (else
      (`self.K2_EndAbility`))))

(fn `GroundAttackDamage`
  (bind _asbp_verina_character (cast `/Game/_BP/YHG/Characters/Verina/BP_VerinaCharacter` (`self.GetPlayerCharacterFromActorInfo`)))
  (bind _returnvalue (`WWObjectPoolComponent.SpawnPooledObject` (`/Game/_BP/YHG/Characters/Verina/BP_VerinaCharacter.VerinaBoxCollision` _asbp_verina_character) _asbp_verina_character))
  (bind _asbp_verina_box_collision (cast `/Game/_BP/YHG/Characters/Verina/AttackCollisionBP/BP_VerinaBoxCollision` _returnvalue))
  (bind _applyattack_basevalue (break `GameplayAttributeData` (`PlayerCharacterAttributeSet.ApplyAttack` (`PlayerCharacter.PlayerCharacterAttributeSet` _asbp_verina_character))))
  (`AttackCollisionBox.InitializeAndAttackWithBoxMultipleEffects` :`self` _asbp_verina_box_collision :`Duration` 2.5 :`BoxExtent` (512.0 512.0 512.0) :`Location` (`Actor.K2_GetActorLocation` _asbp_verina_character) :`InGameplayEffectSpecHandles` (`|MakeArray` (`self.MakePlayerDamageGameplayEffectSpecHandle` "/Game/_BP/JMS/Character/AbilitySystem/GE/GE_Damaged_Enemy.GE_Damaged_Enemy_C" _applyattack_basevalue (struct :`TagName` "Shared.SetByCaller.Damage.Light")) (`self.MakePlayerDamageGameplayEffectSpecHandle` "/Game/_BP/JMS/Character/AbilitySystem/GE/GE_Damaged_Enemy.GE_Damaged_Enemy_C" (* _applyattack_basevalue 10.0) (struct :`TagName` "Shared.SetByCaller.Damage.Stagger")) (`self.MakePlayerDamageGameplayEffectSpecHandle` "/Game/_BP/JMS/Character/AbilitySystem/GE/GE_Damaged_Enemy.GE_Damaged_Enemy_C" _applyattack_basevalue (struct :`TagName` "Shared.SetByCaller.Damage.Parry"))) :`InHitReactEventTag` (struct :`TagName` "Shared.Event.HitReact.Big")))

(fn `RotateEnemyDirection`
  (bind _returnvalue (`self.GetPlayerCharacterFromActorInfo`))
  (bind _asbp_wwplayer_controller (cast `/Game/_BP/YHG/PlayerControllers/BP_WWPlayerController` (`self.GetPlayerControllerFromActorInfo`)))
  (bind _closestenemy (`/Game/_BP/YHG/PlayerControllers/BP_WWPlayerController.ClosestEnemy` _asbp_wwplayer_controller))
  (`/Engine/EditorBlueprintResources/StandardMacros.IsValid` _closestenemy
    (:`Is Valid`
      (bind (_returnvalue_roll _returnvalue_pitch _returnvalue_yaw) (`KismetMathLibrary.BreakRotator` (`KismetMathLibrary.FindLookAtRotation` (`Actor.K2_GetActorLocation` _returnvalue) (`Actor.K2_GetActorLocation` _closestenemy))))
      (`Actor.K2_SetActorRotation` _returnvalue (`KismetMathLibrary.MakeRotator` 0.0 0.0 _returnvalue_yaw) true))))

(fn `RotateMoveDirection`
  (bind _followcamera (`PlayerCharacter.FollowCamera` (`self.GetPlayerCharacterFromActorInfo`)))
  (bind (_returnvalue_x _returnvalue_y) (`KismetMathLibrary.BreakVector` (`SceneComponent.GetRightVector` _followcamera)))
  (bind (_x _y) (`KismetMathLibrary.BreakVector2D` (`WWPlayerController.IsInputMove` (`self.GetPlayerControllerFromActorInfo`))))
  (bind (_returnvalue_x_2 _returnvalue_y_2) (`KismetMathLibrary.BreakVector` (`SceneComponent.GetForwardVector` _followcamera)))
  (bind _returnvalue (+ (* (`KismetMathLibrary.Normal` (`KismetMathLibrary.MakeVector` _returnvalue_x _returnvalue_y)) _x) (* (`KismetMathLibrary.Normal` (`KismetMathLibrary.MakeVector` _returnvalue_x_2 _returnvalue_y_2)) _y)))
  (if (`KismetMathLibrary.NotEqualExactly_VectorVector` _returnvalue)
    (`Actor.K2_SetActorRotation` (`self.GetPlayerCharacterFromActorInfo`) (`KismetMathLibrary.MakeRotFromX` _returnvalue) true)))