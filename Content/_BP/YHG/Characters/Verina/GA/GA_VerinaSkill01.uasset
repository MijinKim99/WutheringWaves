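; Gameplay Ability for Verina's grounded E skill, a ranged attack that ends immediately when airborne.
; It starts the HUD and ability cooldowns, turns her toward camera-relative input, overridden by any closest enemy, then plays the skill montage.
; As the montage starts, a pooled box projectile fires, at that enemy if valid, carrying attack-scaled light, stagger and parry damage effects.
; The Rectifier weapon shows during the skill and hides on ability end.
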(event `self.K2_ActivateAbility`
  (bind _returnvalue (`self.GetPlayerCharacterFromActorInfo`))
  (if (`PlayerCharacter.bIsGrounded` (`self.GetPlayerCharacterFromActorInfo`))
    (bind _asbp_wwplayer_controller (cast `/Game/_BP/YHG/PlayerControllers/BP_WWPlayerController` (`GameplayStatics.GetPlayerController` 0)))
    (`/Game/_BP/KMJ/Widget/HUD/Assets/WBP_SkillIcon_E.CoolTimeEvent` (`/Game/_BP/KMJ/Widget/HUD/WBP_PlayerHUD.WBP_SkillIcon_E_Verina` (`/Game/_BP/YHG/PlayerControllers/BP_WWPlayerController.Widget_PlayerHUD` _asbp_wwplayer_controller)) 12.0)
    (`self.K2_CommitAbilityCooldown` false)
    (`self.RotateMoveDirection`)
    (`self.RotateEnemyDirection`)
    (set `PlayerCharacter.bSprintMode` false _returnvalue)
    (set `PlayerCharacter.bAttackMode` true _returnvalue)
    (`AbilityTask_PlayMontageAndWait.CreatePlayMontageAndWaitProxy` "None" "/Game/_BP/YHG/Characters/Verina/Animation/UseAnimation/CharacterAnim/Skill/AM_VerinaAnim_R2T1JueyuanMd10011_Lod4_Skill02_Edited.AM_VerinaAnim_R2T1JueyuanMd10011_Lod4_Skill02_Edited"
      (:`then`
        (`self.GroundAttackDamage`)
        (`self.VisibleWeapon`))
      (:`OnCompleted`
        (`self.K2_EndAbility` :!label _label))
      (:`OnBlendOut`
        (goto _label))
      (:`OnInterrupted`
        (goto _label))
      (:`OnCancelled`
        (goto _label)))
    (else
      (`self.K2_EndAbility`))))

(event `self.K2_OnEndAbility`
  (params (bWasCancelled :type Boolean))
  (`self.HiddenWeapon`))

(fn `GroundAttackDamage`
  (bind _asbp_verina_character (cast `/Game/_BP/YHG/Characters/Verina/BP_VerinaCharacter` (`self.GetPlayerCharacterFromActorInfo`)))
  (bind _returnvalue (`WWObjectPoolComponent.SpawnPooledObject` (`/Game/_BP/YHG/Characters/Verina/BP_VerinaCharacter.VerinaBoxProjectileCollision` _asbp_verina_character) _asbp_verina_character))
  (bind _asbp_verina_box_projectile_collision (cast `/Game/_BP/YHG/Characters/Verina/AttackCollisionBP/BP_VerinaBoxProjectileCollision` _returnvalue))
  (bind _asbp_wwplayer_controller (cast `/Game/_BP/YHG/PlayerControllers/BP_WWPlayerController` (`self.GetPlayerControllerFromActorInfo`)))
  (bind _closestenemy (`/Game/_BP/YHG/PlayerControllers/BP_WWPlayerController.ClosestEnemy` _asbp_wwplayer_controller))
  (`/Engine/EditorBlueprintResources/StandardMacros.IsValid` _closestenemy
    (:`Is Valid`
      (bind _mesh (`Character.Mesh` _asbp_verina_character))
      (bind _applyattack_basevalue (break `GameplayAttributeData` (`PlayerCharacterAttributeSet.ApplyAttack` (`PlayerCharacter.PlayerCharacterAttributeSet` _asbp_verina_character))))
      (bind _array (`|MakeArray` (`self.MakePlayerDamageGameplayEffectSpecHandle` "/Game/_BP/JMS/Character/AbilitySystem/GE/GE_Damaged_Enemy.GE_Damaged_Enemy_C" _applyattack_basevalue (struct :`TagName` "Shared.SetByCaller.Damage.Light")) (`self.MakePlayerDamageGameplayEffectSpecHandle` "/Game/_BP/JMS/Character/AbilitySystem/GE/GE_Damaged_Enemy.GE_Damaged_Enemy_C" (* _applyattack_basevalue 2.0) (struct :`TagName` "Shared.SetByCaller.Damage.Stagger")) (`self.MakePlayerDamageGameplayEffectSpecHandle` "/Game/_BP/JMS/Character/AbilitySystem/GE/GE_Damaged_Enemy.GE_Damaged_Enemy_C" _applyattack_basevalue (struct :`TagName` "Shared.SetByCaller.Damage.Parry"))))
      (`AttackCollisionBoxProjectile.InitializeAttachedProjectileAndShootMultipleEffects` :`self` _asbp_verina_box_projectile_collision :`BoxExtent` (8.0 8.0 8.0) :`InstigatorMesh` _mesh :`AttachSocketName` "Bip001Spine2" :`InGameplayEffectSpecHandles` _array :`TargetLocation` (`Actor.K2_GetActorLocation` _closestenemy) :`ProjectileSpeed` 500000.0 :`InHitReactEventTag` (struct :`TagName` "Shared.Event.HitReact.Small") :`bShowCollisionInGame` true :`LineThickness` 5.0))
    (:`Is Not Valid`
      (`AttackCollisionBoxProjectile.InitializeAttachedProjectileAndShootMultipleEffects` :`self` _asbp_verina_box_projectile_collision :`BoxExtent` (8.0 8.0 8.0) :`InstigatorMesh` _mesh :`AttachSocketName` "Bip001Spine2" :`InGameplayEffectSpecHandles` _array :`ProjectileSpeed` 500000.0 :`InHitReactEventTag` (struct :`TagName` "Shared.Event.HitReact.Small") :`bShowCollisionInGame` true :`LineThickness` 5.0))))

(fn `HiddenWeapon`
  (bind _asbp_verina_character (cast `/Game/_BP/YHG/Characters/Verina/BP_VerinaCharacter` (`self.GetPlayerCharacterFromActorInfo`)))
  (`SceneComponent.SetVisibility` (`/Game/_BP/YHG/Characters/Verina/BP_VerinaCharacter.Rectifier` _asbp_verina_character) false false))

(fn `RotateEnemyDirection`
  (bind _returnvalue (`self.GetPlayerCharacterFromActorInfo`))
  (bind _asbp_wwplayer_controller (cast `/Game/_BP/YHG/PlayerControllers/BP_WWPlayerController` (`self.GetPlayerControllerFromActorInfo`)))
  (bind _closestenemy (`/Game/_BP/YHG/PlayerControllers/BP_WWPlayerController.ClosestEnemy` _asbp_wwplayer_controller))
  (`/Engine/EditorBlueprintResources/StandardMacros.IsValid` _closestenemy
    (:`Is Valid`
      (bind (_returnvalue_roll _returnvalue_pitch _returnvalue_yaw) (`KismetMathLibrary.BreakRotator` (`KismetMathLibrary.FindLookAtRotation` (`Actor.K2_GetActorLocation` _returnvalue) (`Actor.K2_GetActorLocation` _closestenemy))))
      (`Actor.K2_SetActorRotation` _returnvalue (`KismetMathLibrary.MakeRotator` 0.0 0.0 _returnvalue_yaw) true))))

(fn `RotateMoveDirection`
  (bind _followcamera (`PlayerCharacter.FollowCamera` (`self.GetPlayerCharacterFromActorInfo`)))
  (bind (_returnvalue_x _returnvalue_y) (`KismetMathLibrary.BreakVector` (`SceneComponent.GetRightVector` _followcamera)))
  (bind (_x _y) (`KismetMathLibrary.BreakVector2D` (`WWPlayerController.IsInputMove` (`self.GetPlayerControllerFromActorInfo`))))
  (bind (_returnvalue_x_2 _returnvalue_y_2) (`KismetMathLibrary.BreakVector` (`SceneComponent.GetForwardVector` _followcamera)))
  (bind _returnvalue (+ (* (`KismetMathLibrary.Normal` (`KismetMathLibrary.MakeVector` _returnvalue_x _returnvalue_y)) _x) (* (`KismetMathLibrary.Normal` (`KismetMathLibrary.MakeVector` _returnvalue_x_2 _returnvalue_y_2)) _y)))
  (if (`KismetMathLibrary.NotEqualExactly_VectorVector` _returnvalue)
    (`Actor.K2_SetActorRotation` (`self.GetPlayerCharacterFromActorInfo`) (`KismetMathLibrary.MakeRotFromX` _returnvalue) true)))

(fn `VisibleWeapon`
  (bind _asbp_verina_character (cast `/Game/_BP/YHG/Characters/Verina/BP_VerinaCharacter` (`self.GetPlayerCharacterFromActorInfo`)))
  (`SceneComponent.SetVisibility` (`/Game/_BP/YHG/Characters/Verina/BP_VerinaCharacter.Rectifier` _asbp_verina_character) true false))