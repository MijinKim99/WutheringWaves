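; Gameplay ability for Verina's light attack: a grounded montage combo that hands off to GA_VerinaAirAttack when airborne and the combo count is low.
; Each press faces camera-relative input, then the closest enemy, plays that step's montage and advances the count, which resets shortly after the montage ends.
; A hit gameplay event triggers a delayed pooled box projectile carrying light, stagger and parry damage, aimed at the closest enemy if valid.
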(event `self.K2_ActivateAbility`
  (bind _returnvalue (`self.GetPlayerCharacterFromActorInfo`))
  (bind _returnvalue_2 (`self.GetPlayerCharacterFromActorInfo`))
  (if (`PlayerCharacter.bIsGrounded` _returnvalue)
    ;[1 1 1] 공중공격을 구현해야하기에, 애니메이션 캔슬되는 거 놔둠
    (`self.VisibleWeapon`)
    (`self.RotateMoveDirection`)
    (`self.RotateEnemyDirection`)
    (`KismetSystemLibrary.K2_ClearAndInvalidateTimerHandle` (`self.ResetTimerHandle`))
    (set `self.CachedComboCount` (`PlayerCharacter.LightAttackComboCount` (`self.GetPlayerCharacterFromActorInfo`)))
    (`AbilityTask_PlayMontageAndWait.CreatePlayMontageAndWaitProxy` "None" (`BlueprintMapLibrary.Map_Find` (`self.AttackMontageMap`) (`PlayerCharacter.LightAttackComboCount` (`self.GetPlayerCharacterFromActorInfo`)))
      (:`then`
        (`|ExecutionSequence`
          (:`then_0`
            (if (== (`PlayerCharacter.LightAttackComboCount` (`self.GetPlayerCharacterFromActorInfo`)) (`BlueprintMapLibrary.Map_Length` (`self.AttackMontageMap`)))
              (`self.ResetComboCount`)
              (else
                (`/Engine/EditorBlueprintResources/StandardMacros.IncrementInt` (`PlayerCharacter.LightAttackComboCount` (`self.GetPlayerCharacterFromActorInfo`))))))
          (:`then_1`
            (set `PlayerCharacter.bAttackMode` true _returnvalue_2)
            (set `PlayerCharacter.bSprintMode` false _returnvalue_2))
          (:`then_2`
            (`AbilityTask_WaitGameplayEvent.WaitGameplayEvent` (struct :`TagName` "Player.Event.HitEnemy") null
              (:`EventReceived`
                (`KismetSystemLibrary.K2_SetTimerDelegate` (delegate `OnGroundAttackCollision`) 0.05))))))
      (:`OnCompleted`
        (`self.K2_EndAbility` :!label _label)
        (bind _returnvalue_3 (`KismetSystemLibrary.K2_SetTimerDelegate` (delegate `ResetComboCount`) 0.25))
        (set `self.ResetTimerHandle` _returnvalue_3))
      (:`OnBlendOut`
        (goto _label))
      (:`OnInterrupted`
        (goto _label))
      (:`OnCancelled`
        (goto _label)))
    (else
      (bind _asbp_verina_character (cast `/Game/_BP/YHG/Characters/Verina/BP_VerinaCharacter` _returnvalue))
      (if (< (`PlayerCharacter.LightAttackComboCount` _asbp_verina_character) 3)
        (`self.VisibleWeapon`)
        (`self.RotateMoveDirection`)
        (`self.RotateEnemyDirection`)
        (`self.ResetComboCount`)
        (`AbilitySystemComponent.TryActivateAbilityByClass` (`self.GetWWAbilitySystemComponentFromActorInfo`) "/Game/_BP/YHG/Characters/Verina/GA/GA_VerinaAirAttack.GA_VerinaAirAttack_C" true)
        (`self.K2_EndAbility`)))))

(event `self.K2_OnEndAbility`
  (params (bWasCancelled :type Boolean)))

(event `OnGroundAttackCollision`
  (`self.GroundAttackDamage`))

(event `ResetComboCount`
  (set `PlayerCharacter.LightAttackComboCount` 1 (`self.GetPlayerCharacterFromActorInfo`)))

(fn `GroundAttackDamage`
  (bind _array (`|MakeArray` (`self.MakePlayerDamageGameplayEffectSpecHandle` "/Game/_BP/JMS/Character/AbilitySystem/GE/GE_Damaged_Enemy.GE_Damaged_Enemy_C" 5.0 (struct :`TagName` "Shared.SetByCaller.Damage.Light")) (`self.MakePlayerDamageGameplayEffectSpecHandle` "/Game/_BP/JMS/Character/AbilitySystem/GE/GE_Damaged_Enemy.GE_Damaged_Enemy_C" 10.0 (struct :`TagName` "Shared.SetByCaller.Damage.Stagger")) (`self.MakePlayerDamageGameplayEffectSpecHandle` "/Game/_BP/JMS/Character/AbilitySystem/GE/GE_Damaged_Enemy.GE_Damaged_Enemy_C" 7.5 (struct :`TagName` "Shared.SetByCaller.Damage.Parry"))))
  (bind _asbp_verina_character (cast `/Game/_BP/YHG/Characters/Verina/BP_VerinaCharacter` (`self.GetPlayerCharacterFromActorInfo`)))
  (bind _returnvalue (`WWObjectPoolComponent.SpawnPooledObject` (`/Game/_BP/YHG/Characters/Verina/BP_VerinaCharacter.VerinaBoxProjectileCollision` _asbp_verina_character) _asbp_verina_character))
  (bind _asbp_verina_box_projectile_collision (cast `/Game/_BP/YHG/Characters/Verina/AttackCollisionBP/BP_VerinaBoxProjectileCollision` _returnvalue))
  (bind _asbp_wwplayer_controller (cast `/Game/_BP/YHG/PlayerControllers/BP_WWPlayerController` (`self.GetPlayerControllerFromActorInfo`)))
  (bind _closestenemy (`/Game/_BP/YHG/PlayerControllers/BP_WWPlayerController.ClosestEnemy` _asbp_wwplayer_controller))
  (`/Engine/EditorBlueprintResources/StandardMacros.IsValid` _closestenemy
    (:`Is Valid`
      (bind _mesh (`Character.Mesh` _asbp_verina_character))
      (`AttackCollisionBoxProjectile.InitializeAttachedProjectileAndShootMultipleEffects` :`self` _asbp_verina_box_projectile_collision :`BoxExtent` (8.0 8.0 8.0) :`InstigatorMesh` _mesh :`AttachSocketName` "Bip001Spine2" :`InGameplayEffectSpecHandles` _array :`TargetLocation` (`Actor.K2_GetActorLocation` _closestenemy) :`ProjectileSpeed` 500000.0 :`InExplosionGameplayCueTag` (struct :`TagName` "GameplayCue.FX.Player.Verina.LightAttack") :`InHitReactEventTag` (struct :`TagName` "Shared.Event.HitReact.Small") :`bShowCollisionInGame` true :`LineThickness` 5.0 :`InbExplodeOnHit` true))
    (:`Is Not Valid`
      (`AttackCollisionBoxProjectile.InitializeAttachedProjectileAndShootMultipleEffects` :`self` _asbp_verina_box_projectile_collision :`BoxExtent` (8.0 8.0 8.0) :`InstigatorMesh` _mesh :`AttachSocketName` "Bip001Spine2" :`InGameplayEffectSpecHandles` _array :`ProjectileSpeed` 500000.0 :`InExplosionGameplayCueTag` (struct :`TagName` "GameplayCue.FX.Player.Verina.LightAttack") :`InHitReactEventTag` (struct :`TagName` "Shared.Event.HitReact.Small") :`bShowCollisionInGame` true :`LineThickness` 5.0 :`InbExplodeOnHit` true))))

(fn `HiddenWeapon`
  (bind _asbp_verina_character (cast `/Game/_BP/YHG/Characters/Verina/BP_VerinaCharacter` (`self.GetPlayerCharacterFromActorInfo`)))
  (`SceneComponent.SetVisibility` (`/Game/_BP/YHG/Characters/Verina/BP_VerinaCharacter.Rectifier` _asbp_verina_character) false false))

(fn `RotateEnemyDirection`
  (bind _returnvalue (`self.GetPlayerCharacterFromActorInfo`))
  (bind _asbp_wwplayer_controller (cast `/Game/_BP/YHG/PlayerControllers/BP_WWPlayerController` (`self.GetPlayerControllerFromActorInfo`)))
  (bind _closestenemy (`/Game/_BP/YHG/PlayerControllers/BP_WWPlayerController.ClosestEnemy` _asbp_wwplayer_controller))
  (`/Engine/EditorBlueprintResources/StandardMacros.IsValid` _closestenemy
    (:`Is Valid`
      (bind (_returnvalue_roll _returnvalue_pitch _returnvalue_yaw) (`KismetMathLibrary.BreakRotator` (`KismetMathLibrary.FindLookAtRotation` (`Actor.K2_GetActorLocation` _returnvalue) (`Actor.K2_GetActorLocation` _closestenemy))))
      (`Actor.K2_SetActorRotation` _returnvalue (`KismetMathLibrary.MakeRotator` 0.0 0.0 _returnvalue_yaw) true))))

(fn `RotateMoveDirection`
  (bind _followcamera (`PlayerCharacter.FollowCamera` (`self.GetPlayerCharacterFromActorInfo`)))
  (bind (_returnvalue_x _returnvalue_y) (`KismetMathLibrary.BreakVector` (`SceneComponent.GetRightVector` _followcamera)))
  (bind (_x _y) (`KismetMathLibrary.BreakVector2D` (`WWPlayerController.IsInputMove` (`self.GetPlayerControllerFromActorInfo`))))
  (bind (_returnvalue_x_2 _returnvalue_y_2) (`KismetMathLibrary.BreakVector` (`SceneComponent.GetForwardVector` _followcamera)))
  (bind _returnvalue (+ (* (`KismetMathLibrary.Normal` (`KismetMathLibrary.MakeVector` _returnvalue_x _returnvalue_y)) _x) (* (`KismetMathLibrary.Normal` (`KismetMathLibrary.MakeVector` _returnvalue_x_2 _returnvalue_y_2)) _y)))
  (if (`KismetMathLibrary.NotEqualExactly_VectorVector` _returnvalue)
    (`Actor.K2_SetActorRotation` (`self.GetPlayerCharacterFromActorInfo`) (`KismetMathLibrary.MakeRotFromX` _returnvalue) true)))

(fn `VisibleWeapon`
  (bind _asbp_verina_character (cast `/Game/_BP/YHG/Characters/Verina/BP_VerinaCharacter` (`self.GetPlayerCharacterFromActorInfo`)))
  (`SceneComponent.SetVisibility` (`/Game/_BP/YHG/Characters/Verina/BP_VerinaCharacter.Rectifier` _asbp_verina_character) true false))