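; Playable Verina character Blueprint that sets up her starting attributes and resets her air combo.
; BeginPlay hides the Rectifier and runs attribute initialization, covering health, combat stats, skill and burst cooldowns, and energy gauges.
; Possession repeats that initialization until VerinaInitialize is set, which requires a BP_WWPlayerController with a valid PlayerState; BeginPlay bypasses this flag check.
; Tick zeroes the air combo count while grounded.
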(event `self.ReceivePossessed`
  (params (NewController :type "Controller Object Reference"))
  (`parent.ReceivePossessed` NewController)
  (if (not (`self.VerinaInitialize`))
    (`self.InitializeAttributeSet` 569.5 1139.0 47.0 47.0 90.0 90.0 100.0 100.0 5.0 5.0 150.0 150.0 12.0 12.0 25.0 25.0 175.0 175.0 100.0 100.0 100.0 100.0 :!label _label)
    (bind _asbp_wwplayer_controller (cast `/Game/_BP/YHG/PlayerControllers/BP_WWPlayerController` (`self.GetController`)))
    (`/Engine/EditorBlueprintResources/StandardMacros.IsValid` (`Controller.PlayerState` _asbp_wwplayer_controller)
      (:`Is Valid`
        (set `self.VerinaInitialize` true)))))

(event `self.ReceiveBeginPlay`
  (`SceneComponent.SetVisibility` (`self.Rectifier`) false false)
  (goto _label))

(event `self.ReceiveTick`
  (params (DeltaSeconds :type "Float (single-precision)"))
  (`parent.ReceiveTick` DeltaSeconds)
  (if (`self.bIsGrounded`)
    (set `self.VerinaAirComboCount` 0)))

(fn `UserConstructionScript`)