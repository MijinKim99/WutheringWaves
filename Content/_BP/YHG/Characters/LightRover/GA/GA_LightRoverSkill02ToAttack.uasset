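; Gameplay ability for the LightRover player character's grounded attack out of Skill02, judging by its name.
; It plays an attack montage and waits for the HitEnemy gameplay event to spawn a pooled box collision at the character.
; The box briefly applies light, stagger and parry damage effects with a small hit react.
; The ability ends when the montage finishes or breaks off, but has no EndAbility path when airborne.
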(event `self.K2_ActivateAbility`
  (if (`PlayerCharacter.bIsGrounded` (`self.GetPlayerCharacterFromActorInfo`))
    (`AbilityTask_PlayMontageAndWait.CreatePlayMontageAndWaitProxy` "None" "/Game/_BP/YHG/Characters/LightRover/Animation/UseAnimation/CharacterAnim/Skill/AM_LightRoverAnim_R2T1PlayerMaleMd10011_Lod4_Attack05_Edited.AM_LightRoverAnim_R2T1PlayerMaleMd10011_Lod4_Attack05_Edited"
      (:`then`
        (`AbilityTask_WaitGameplayEvent.WaitGameplayEvent` (struct :`TagName` "Player.Event.HitEnemy") null
          (:`EventReceived`
            (bind _asbp_light_rover_character (cast `/Game/_BP/YHG/Characters/LightRover/BP_LightRoverCharacter` (`self.GetPlayerCharacterFromActorInfo`)))
            (bind _returnvalue (`WWObjectPoolComponent.SpawnPooledObject` (`/Game/_BP/YHG/Characters/LightRover/BP_LightRoverCharacter.LightRoverBoxCollision` _asbp_light_rover_character) _asbp_light_rover_character))
            (bind _asbp_light_rover_box_collision (cast `/Game/_BP/YHG/Characters/LightRover/AttackCollisionBP/BP_LightRoverBoxCollision` _returnvalue))
            (`AttackCollisionBox.InitializeAndAttackWithBoxMultipleEffects` :`self` _asbp_light_rover_box_collision :`Duration` 0.125 :`BoxExtent` (128.0 128.0 128.0) :`Location` (`Actor.K2_GetActorLocation` _asbp_light_rover_character) :`InGameplayEffectSpecHandles` (`|MakeArray` (`self.MakePlayerDamageGameplayEffectSpecHandle` "/Game/_BP/JMS/Character/AbilitySystem/GE/GE_Damaged_Enemy.GE_Damaged_Enemy_C" 15.0 (struct :`TagName` "Shared.SetByCaller.Damage.Light")) (`self.MakePlayerDamageGameplayEffectSpecHandle` "/Game/_BP/JMS/Character/AbilitySystem/GE/GE_Damaged_Enemy.GE_Damaged_Enemy_C" 15.0 (struct :`TagName` "Shared.SetByCaller.Damage.Stagger")) (`self.MakePlayerDamageGameplayEffectSpecHandle` "/Game/_BP/JMS/Character/AbilitySystem/GE/GE_Damaged_Enemy.GE_Damaged_Enemy_C" 20.0 (struct :`TagName` "Shared.SetByCaller.Damage.Parry"))) :`InHitReactEventTag` (struct :`TagName` "Shared.Event.HitReact.Small")))))
      (:`OnCompleted`
        (`self.K2_EndAbility` :!label _label))
      (:`OnBlendOut`
        (goto _label))
      (:`OnInterrupted`
        (goto _label))
      (:`OnCancelled`
        (goto _label)))))