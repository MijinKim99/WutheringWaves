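; Gameplay ability for LightRover's first skill, which works only while the character is grounded.
; On activation it commits the cooldown, turns off sprint mode and checks an ability-system attribute against a threshold.
; At or above the threshold it hands off to GA_LightRoverSkill02 and ends.
; Otherwise it plays the Skill01 montage and ends when that completes, blends out or is stopped.
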(event `self.K2_ActivateAbility`
  (bind (_bsuccessfullyfoundattribute _returnvalue) (`AbilitySystemBlueprintLibrary.GetFloatAttributeFromAbilitySystemComponent` (`self.GetWWAbilitySystemComponentFromActorInfo`) (struct :`AttributeName` "CurrentForteCircuitEnergy" :`Attribute` "/Script/WutheringWaves.PlayerCharacterAttributeSet:CurrentForteCircuitEnergy" :`AttributeOwner` "/Script/CoreUObject.Class'/Script/WutheringWaves.PlayerCharacterAttributeSet'")))
  (if (`PlayerCharacter.bIsGrounded` (`self.GetPlayerCharacterFromActorInfo`))
    (`self.K2_CommitAbilityCooldown` false)
    (set `PlayerCharacter.bSprintMode` false (`self.GetPlayerCharacterFromActorInfo`))
    (if (and _bsuccessfullyfoundattribute (>= _returnvalue 50.0))
      (`AbilitySystemComponent.TryActivateAbilityByClass` (`self.GetWWAbilitySystemComponentFromActorInfo`) "/Game/_BP/YHG/Characters/LightRover/GA/GA_LightRoverSkill02.GA_LightRoverSkill02_C" true)
      (`self.K2_EndAbility`)
      (else
        (`AbilityTask_PlayMontageAndWait.CreatePlayMontageAndWaitProxy` "None" "/Game/_BP/YHG/Characters/LightRover/Animation/UseAnimation/CharacterAnim/Skill/AM_LightRoverAnim_R2T1PlayerMaleMd10011_Lod4_Skill01_Edited.AM_LightRoverAnim_R2T1PlayerMaleMd10011_Lod4_Skill01_Edited"
          (:`OnCompleted`
            _)
          (:`OnBlendOut`
            _)
          (:`OnInterrupted`
            _)
          (:`OnCancelled`
            _))
        (`self.K2_EndAbility`)))
    (else
      (`self.K2_EndAbility`))))