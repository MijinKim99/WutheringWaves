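; BP_LightRoverCharacter is the Light Rover playable character, configured with its starting combat stats and sword equipment.
; On BeginPlay it hides the sword and scabbard, disables sword collision, and initializes an attribute set covering health, combat stats, skill and burst cooldowns, and energy gauges.
; It then links Rover to the player HUD through BP_WWPlayerController.
; Tick only calls the parent implementation.
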(event `self.ReceiveBeginPlay`
  (`|ExecutionSequence`
    (:`then_0`
      (`SceneComponent.SetVisibility` (`self.Scabbard`) false false)
      (`SceneComponent.SetVisibility` (`self.Sword`) false false)
      (`self.InitializeAttributeSet` 50.0 50.0 30.0 30.0 112.0 112.0 100.0 100.0 5.0 5.0 150.0 150.0 5.0 5.0 19.0 19.0 125.0 125.0 100.0 100.0 100.0 100.0)
      (bind _asbp_wwplayer_controller (cast `/Game/_BP/YHG/PlayerControllers/BP_WWPlayerController` (`self.GetController`)))
      (`/Game/_BP/KMJ/Widget/HUD/WBP_PlayerHUD.LinkPawnToUI` (`/Game/_BP/YHG/PlayerControllers/BP_WWPlayerController.Widget_PlayerHUD` _asbp_wwplayer_controller) "Rover"))
    (:`then_1`
      (`PrimitiveComponent.SetCollisionEnabled` (`self.Sword`) "NoCollision"))))

(event `self.ReceiveTick`
  (params (DeltaSeconds :type "Float (single-precision)"))
  (`parent.ReceiveTick` DeltaSeconds))

(fn `UserConstructionScript`)