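; Gameplay ability for Chixia's air attack, which alternates between two montages on each activation and zeroes her velocity to stall her in the air.
; While active it sets attack mode, and each HitEnemy gameplay event fires a pooled box projectile from her current attack socket.
; The projectile carries Fire and Stagger damage effects with a small hit react, and is aimed at the controller's closest enemy when one is valid.
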(event `self.K2_ActivateAbility`
  (`self.K2_CommitAbilityCost` false)
  (if (`self.ShootHand`)
    (set `self.ShootHand` false)
    (`AbilityTask_PlayMontageAndWait.CreatePlayMontageAndWaitProxy` "None" "/Game/_BP/YHG/Characters/Chixia/Animation/UseAnimation/CharacterAnim/Attack/AM_ChixiaAnim_R2T1MaxiaofangMd10011_Lod4_AirAttack01_Fl_Edited.AM_ChixiaAnim_R2T1MaxiaofangMd10011_Lod4_AirAttack01_Fl_Edited"
      (:`then`
        (set `MovementComponent.Velocity` (0.0 0.0 0.0) (`Character.CharacterMovement` (`self.GetPlayerCharacterFromActorInfo`)) :!label _label)
        (`AbilityTask_WaitGameplayEvent.WaitGameplayEvent` (struct :`TagName` "Player.Event.HitEnemy") null
          (:`then`
            (set `PlayerCharacter.bAttackMode` true (`self.GetPlayerCharacterFromActorInfo`)))
          (:`EventReceived`
            (`self.AirAttackDamage`))))
      (:`OnCompleted`
        (`self.K2_EndAbility` :!label _label_2))
      (:`OnBlendOut`
        (goto _label_2))
      (:`OnInterrupted`
        (goto _label_2))
      (:`OnCancelled`
        (goto _label_2)))
    (else
      (set `self.ShootHand` true)
      (`AbilityTask_PlayMontageAndWait.CreatePlayMontageAndWaitProxy` "None" "/Game/_BP/YHG/Characters/Chixia/Animation/UseAnimation/CharacterAnim/Attack/AM_ChixiaAnim_R2T1MaxiaofangMd10011_Lod4_AirAttack01_FR_Edited.AM_ChixiaAnim_R2T1MaxiaofangMd10011_Lod4_AirAttack01_FR_Edited"
        (:`then`
          (goto _label))
        (:`OnCompleted`
          _)
        (:`OnBlendOut`
          _)
        (:`OnInterrupted`
          _)
        (:`OnCancelled`
          _))
      (`self.K2_EndAbility`))))

(fn `AirAttackDamage`
  (bind _asbp_chixia_character (cast `/Game/_BP/YHG/Characters/Chixia/BP_ChixiaCharacter` (`self.GetPlayerCharacterFromActorInfo`)))
  (bind _returnvalue (`WWObjectPoolComponent.SpawnPooledObject` (`/Game/_BP/YHG/Characters/Chixia/BP_ChixiaCharacter.ChixiaBoxProjectileCollision` _asbp_chixia_character) _asbp_chixia_character))
  (bind _asbp_chixia_box_projectile_collision (cast `/Game/_BP/YHG/Characters/Chixia/AttackCollisionBP/BP_ChixiaBoxProjectileCollision` _returnvalue))
  (bind _asbp_wwplayer_controller (cast `/Game/_BP/YHG/PlayerControllers/BP_WWPlayerController` (`self.GetPlayerControllerFromActorInfo`)))
  (bind _closestenemy (`/Game/_BP/YHG/PlayerControllers/BP_WWPlayerController.ClosestEnemy` _asbp_wwplayer_controller))
  (`/Engine/EditorBlueprintResources/StandardMacros.IsValid` _closestenemy
    (:`Is Valid`
      (bind _mesh (`Character.Mesh` _asbp_chixia_character))
      (bind _currentattacksocket (`/Game/_BP/YHG/Characters/Chixia/BP_ChixiaCharacter.CurrentAttackSocket` _asbp_chixia_character))
      (bind _applyattack_basevalue (break `GameplayAttributeData` (`PlayerCharacterAttributeSet.ApplyAttack` (`PlayerCharacter.PlayerCharacterAttributeSet` _asbp_chixia_character))))
      (bind _array (`|MakeArray` (`self.MakePlayerDamageGameplayEffectSpecHandle` "/Game/_BP/JMS/Character/AbilitySystem/GE/GE_Damaged_Enemy.GE_Damaged_Enemy_C" _applyattack_basevalue (struct :`TagName` "Shared.SetByCaller.Damage.Fire")) (`self.MakePlayerDamageGameplayEffectSpecHandle` "/Game/_BP/JMS/Character/AbilitySystem/GE/GE_Damaged_Enemy.GE_Damaged_Enemy_C" _applyattack_basevalue (struct :`TagName` "Shared.SetByCaller.Damage.Stagger"))))
      (`AttackCollisionBoxProjectile.InitializeAttachedProjectileAndShootMultipleEffects` :`self` _asbp_chixia_box_projectile_collision :`BoxExtent` (8.0 8.0 8.0) :`InstigatorMesh` _mesh :`AttachSocketName` _currentattacksocket :`InGameplayEffectSpecHandles` _array :`TargetLocation` (`Actor.K2_GetActorLocation` _closestenemy) :`ProjectileSpeed` 500000.0 :`InHitReactEventTag` (struct :`TagName` "Shared.Event.HitReact.Small") :`bShowCollisionInGame` true :`LineThickness` 5.0))
    (:`Is Not Valid`
      (`AttackCollisionBoxProjectile.InitializeAttachedProjectileAndShootMultipleEffects` :`self` _asbp_chixia_box_projectile_collision :`BoxExtent` (8.0 8.0 8.0) :`InstigatorMesh` _mesh :`AttachSocketName` _currentattacksocket :`InGameplayEffectSpecHandles` _array :`ProjectileSpeed` 500000.0 :`InHitReactEventTag` (struct :`TagName` "Shared.Event.HitReact.Small") :`bShowCollisionInGame` true :`LineThickness` 5.0))))