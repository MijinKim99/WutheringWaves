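; Gameplay ability for Chixia's Burst skill, a grounded-only area attack dealing fire and stagger damage.
; It starts the HUD cooldown, commits cooldown and cost, then faces move input, overridden by the closest enemy if valid.
; During the montage it switches to attack mode, and each HitEnemy gameplay event spawns a pooled box collision around her, applying attack-scaled damage effects and small hit reacts.
; The ability ends when the montage finishes or is interrupted.
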(event `self.K2_ActivateAbility`
  (bind _returnvalue (`self.GetPlayerCharacterFromActorInfo`))
  (if (`PlayerCharacter.bIsGrounded` (`self.GetPlayerCharacterFromActorInfo`))
    (bind _asbp_wwplayer_controller (cast `/Game/_BP/YHG/PlayerControllers/BP_WWPlayerController` (`GameplayStatics.GetPlayerController` 0)))
    (`/Game/_BP/KMJ/Widget/HUD/Assets/WBP_SkillIcon_R.CoolTimeEvent` (`/Game/_BP/KMJ/Widget/HUD/WBP_PlayerHUD.WBP_SkillIcon_R_Chixia` (`/Game/_BP/YHG/PlayerControllers/BP_WWPlayerController.Widget_PlayerHUD` _asbp_wwplayer_controller)) 20.0)
    (`self.K2_CommitAbilityCooldown` false)
    (`self.K2_CommitAbilityCost` false)
    (`self.RotateMoveDirection`)
    (`self.RotateEnemyDirection`)
    (`AbilityTask_PlayMontageAndWait.CreatePlayMontageAndWaitProxy` "None" "/Game/_BP/YHG/Characters/Chixia/Animation/UseAnimation/CharacterAnim/Burst/AM_ChixiaAnim_R2T1MaxiaofangMd10011_Lod4_Burst01_Edited.AM_ChixiaAnim_R2T1MaxiaofangMd10011_Lod4_Burst01_Edited"
      (:`then`
        (`AbilityTask_WaitGameplayEvent.WaitGameplayEvent` (struct :`TagName` "Player.Event.HitEnemy") null
          (:`then`
            (set `PlayerCharacter.bSprintMode` false _returnvalue)
            (set `PlayerCharacter.bAttackMode` true _returnvalue))
          (:`EventReceived`
            (bind _asbp_chixia_character (cast `/Game/_BP/YHG/Characters/Chixia/BP_ChixiaCharacter` (`self.GetPlayerCharacterFromActorInfo`)))
            (bind _returnvalue_2 (`WWObjectPoolComponent.SpawnPooledObject` (`/Game/_BP/YHG/Characters/Chixia/BP_ChixiaCharacter.ChixiaBoxCollision` _asbp_chixia_character) _asbp_chixia_character))
            (bind _asbp_chixia_box_collision (cast `/Game/_BP/YHG/Characters/Chixia/AttackCollisionBP/BP_ChixiaBoxCollision` _returnvalue_2))
            (bind _applyattack_basevalue (break `GameplayAttributeData` (`PlayerCharacterAttributeSet.ApplyAttack` (`PlayerCharacter.PlayerCharacterAttributeSet` _asbp_chixia_character))))
            (`AttackCollisionBox.InitializeAndAttackWithBoxMultipleEffects` :`self` _asbp_chixia_box_collision :`Duration` 0.125 :`BoxExtent` (256.0 256.0 256.0) :`Location` (`Actor.K2_GetActorLocation` (`self.GetPlayerCharacterFromActorInfo`)) :`InGameplayEffectSpecHandles` (`|MakeArray` (`self.MakePlayerDamageGameplayEffectSpecHandle` "/Game/_BP/JMS/Character/AbilitySystem/GE/GE_Damaged_Enemy.GE_Damaged_Enemy_C" (* _applyattack_basevalue 2.5) (struct :`TagName` "Shared.SetByCaller.Damage.Fire")) (`self.MakePlayerDamageGameplayEffectSpecHandle` "/Game/_BP/JMS/Character/AbilitySystem/GE/GE_Damaged_Enemy.GE_Damaged_Enemy_C" _applyattack_basevalue (struct :`TagName` "Shared.SetByCaller.Damage.Stagger"))) :`InHitReactEventTag` (struct :`TagName` "Shared.Event.HitReact.Small")))))
      (:`OnCompleted`
        (`self.K2_EndAbility` :!label _label))
      (:`OnBlendOut`
        (goto _label))
      (:`OnInterrupted`
        (goto _label))
      (:`OnCancelled`
        (goto _label)))
    (else
      (`self.K2_EndAbility`))))

(fn `RotateEnemyDirection`
  (bind _returnvalue (`self.GetPlayerCharacterFromActorInfo`))
  (bind _asbp_wwplayer_controller (cast `/Game/_BP/YHG/PlayerControllers/BP_WWPlayerController` (`self.GetPlayerControllerFromActorInfo`)))
  (bind _closestenemy (`/Game/_BP/YHG/PlayerControllers/BP_WWPlayerController.ClosestEnemy` _asbp_wwplayer_controller))
  (`/Engine/EditorBlueprintResources/StandardMacros.IsValid` _closestenemy
    (:`Is Valid`
      (bind (_returnvalue_roll _returnvalue_pitch _returnvalue_yaw) (`KismetMathLibrary.BreakRotator` (`KismetMathLibrary.FindLookAtRotation` (`Actor.K2_GetActorLocation` _returnvalue) (`Actor.K2_GetActorLocation` _closestenemy))))
      (`Actor.K2_SetActorRotation` _returnvalue (`KismetMathLibrary.MakeRotator` 0.0 0.0 _returnvalue_yaw) true))))

(fn `RotateMoveDirection`
  (bind _followcamera (`PlayerCharacter.FollowCamera` (`self.GetPlayerCharacterFromActorInfo`)))
  (bind (_returnvalue_x _returnvalue_y) (`KismetMathLibrary.BreakVector` (`SceneComponent.GetRightVector` _followcamera)))
  (bind (_x _y) (`KismetMathLibrary.BreakVector2D` (`WWPlayerController.IsInputMove` (`self.GetPlayerControllerFromActorInfo`))))
  (bind (_returnvalue_x_2 _returnvalue_y_2) (`KismetMathLibrary.BreakVector` (`SceneComponent.GetForwardVector` _followcamera)))
  (bind _returnvalue (+ (* (`KismetMathLibrary.Normal` (`KismetMathLibrary.MakeVector` _returnvalue_x _returnvalue_y)) _x) (* (`KismetMathLibrary.Normal` (`KismetMathLibrary.MakeVector` _returnvalue_x_2 _returnvalue_y_2)) _y)))
  (if (`KismetMathLibrary.NotEqualExactly_VectorVector` _returnvalue)
    (`Actor.K2_SetActorRotation` (`self.GetPlayerCharacterFromActorInfo`) (`KismetMathLibrary.MakeRotFromX` _returnvalue) true)))