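; Gameplay ability for the Celestial Light Rover's grounded light-attack combo.
; On activation it plays the montage mapped to the player controller's combo count, then immediately advances the count, wrapping to one after the last entry.
; When the montage ends or is interrupted, the ability ends and starts a short combo-reset timer, which the next grounded activation clears.
; Activating off the ground resets the combo and ends the ability.
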(event `self.K2_ActivateAbility`
  (if (`NavMovementComponent.IsMovingOnGround` (`Character.CharacterMovement` (`self.GetPlayerCharacterFromActorInfo`)))
    (`KismetSystemLibrary.K2_ClearAndInvalidateTimerHandle` (`self.ResetTimerHandle`))
    (`AbilityTask_PlayMontageAndWait.CreatePlayMontageAndWaitProxy` "None" (`BlueprintMapLibrary.Map_Find` (`self.AttackMontageMap`) (`WWPlayerController.LightAttackComboCount` (`self.GetPlayerControllerFromActorInfo`)))
      (:`then`
        (`|ExecutionSequence`
          (:`then_0`
            (if (== (`WWPlayerController.LightAttackComboCount` (`self.GetPlayerControllerFromActorInfo`)) (`BlueprintMapLibrary.Map_Length` (`self.AttackMontageMap`)))
              (`self.ResetComboCount`)
              (else
                (`/Engine/EditorBlueprintResources/StandardMacros.IncrementInt` (`WWPlayerController.LightAttackComboCount` (`self.GetPlayerControllerFromActorInfo`))))))))
      (:`OnCompleted`
        (`self.K2_EndAbility` :!label _label)
        (bind _returnvalue (`KismetSystemLibrary.K2_SetTimerDelegate` (delegate `ResetComboCount`) 0.5))
        (set `self.ResetTimerHandle` _returnvalue))
      (:`OnBlendOut`
        (goto _label))
      (:`OnInterrupted`
        (goto _label))
      (:`OnCancelled`
        (goto _label)))
    (else
      (`self.ResetComboCount`)
      (`self.K2_EndAbility`))))

(event `ResetComboCount`
  (set `WWPlayerController.LightAttackComboCount` 1 (`self.GetPlayerControllerFromActorInfo`)))