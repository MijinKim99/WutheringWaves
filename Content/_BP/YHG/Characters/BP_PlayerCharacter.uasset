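; Player character Blueprint that handles sprint-stop animation and dash count reset.
; On possession it caches its BP_WWPlayerController, whose move input Tick polls to end sprint on the ground when input is released.
; If no montage is active and velocity points forward, it plays a left or right stop montage based on IsRightMoving.
; Tick also starts a guarded timer at the first counted dash, which clears the dash count as a cooldown.
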(event `self.ReceiveBeginPlay`)

(event `self.ReceivePossessed`
  (params (NewController :type "Controller Object Reference"))
  (bind _asbp_wwplayer_controller (cast `/Game/_BP/YHG/PlayerControllers/BP_WWPlayerController` NewController))
  (set `self.As BP WWPlayer Controller` _asbp_wwplayer_controller))

(event `self.ReceiveTick`
  (params (DeltaSeconds :type "Float (single-precision)"))
  (bind _as_bp_wwplayer_controller (`self.As BP WWPlayer Controller`))
  (set `self.Delta Seconds` DeltaSeconds)
  (`|ExecutionSequence`
    (:`then_0`
      ;[1 1 1] 달리다가 멈추었을 때 재생되는 몽타주로, 다른 몽타주가 있을 때는 재생하지 않는다
      (`/Engine/EditorBlueprintResources/StandardMacros.IsValid` _as_bp_wwplayer_controller
        (:`Is Valid`
          (if (and (`self.bSprintMode`) (`self.bIsGrounded`) (`KismetMathLibrary.IsZero2D` (`WWPlayerController.IsInputMove` _as_bp_wwplayer_controller)))
            (set `self.bSprintMode` false)
            (`/Engine/EditorBlueprintResources/StandardMacros.IsValid` (`AnimInstance.GetCurrentActiveMontage` (`SkeletalMeshComponent.GetAnimInstance` (`self.Mesh`)))
              (:`Is Not Valid`
                (if (> (`KismetMathLibrary.Dot_VectorVector` (`KismetMathLibrary.GetForwardVector` (`self.K2_GetActorRotation`)) (`MovementComponent.Velocity` (`self.CharacterMovement`))) 0.5)
                  (if (`self.bIsRightMoving`)
                    (`self.PlayAnimMontage` (`self.RStopSprint`))
                    (else
                      (`self.PlayAnimMontage` (`self.LStopSprint`)))))))))))
    (:`then_1`
      ;[1 1 1] 대쉬를 연속 2번했을 때, 다시 사용할 수 있는 쿨타임
      (if (and (== (`self.DashCount`) 1) (not (`self.bDashInitCheck`)))
        (set `self.bDashInitCheck` true)
        (`KismetSystemLibrary.K2_SetTimerDelegate` (delegate `ResetDashCount`) 1.5)))))

(event `ResetDashCount`
  ;[1 1 1] 대쉬를 연속 2번했을 때, 다시 사용할 수 있는 쿨타임
  (set `self.bDashInitCheck` false)
  (set `self.DashCount` 0))

(fn `UserConstructionScript`)