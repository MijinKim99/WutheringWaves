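; GA_Dash is a Gameplay Ability that performs the player character's dash, available only while moving on the ground.
; It reads the player controller's IsMove vector, playing the forward dash montage when there is movement input and the backward one otherwise.
; The ability ends when the montage completes, blends out, is interrupted or is cancelled, or immediately if the character is not grounded.
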(event `self.K2_ActivateAbility`
  (if (`NavMovementComponent.IsMovingOnGround` (`Character.CharacterMovement` (`self.GetPlayerCharacterFromActorInfo`)))
    (if (> (`KismetMathLibrary.VSize2D` (`WWPlayerController.IsMove` (`self.GetPlayerControllerFromActorInfo`))) 0.0)
      (`AbilityTask_PlayMontageAndWait.CreatePlayMontageAndWaitProxy` "None" "/Game/_BP/YHG/Characters/CelestialLightRover/Animation/UseAnimation/BasicAnim/Dash/AM_MaleMBaseAnim_R2T1PlayerMaleMd10011_Lod4_Move_F_Edited_Montage.AM_MaleMBaseAnim_R2T1PlayerMaleMd10011_Lod4_Move_F_Edited_Montage"
        (:`OnCompleted`
          _)
        (:`OnBlendOut`
          _)
        (:`OnInterrupted`
          _)
        (:`OnCancelled`
          _))
      (`self.K2_EndAbility`)
      (else
        (`AbilityTask_PlayMontageAndWait.CreatePlayMontageAndWaitProxy` "None" "/Game/_BP/YHG/Characters/CelestialLightRover/Animation/UseAnimation/BasicAnim/Dash/AM_MaleMBaseAnim_R2T1PlayerMaleMd10011_Lod4_Move_B_Edited_Montage.AM_MaleMBaseAnim_R2T1PlayerMaleMd10011_Lod4_Move_B_Edited_Montage"
          (:`OnCompleted`
            _)
          (:`OnBlendOut`
            _)
          (:`OnInterrupted`
            _)
          (:`OnCancelled`
            _))
        (`self.K2_EndAbility`)))
    (else
      (`self.K2_EndAbility`))))