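; GA_Jump is a Gameplay Ability that makes the player character perform a short jump press, only while moving on the ground.
; Before jumping, it zeroes velocity when the controller's IsMove input is zero, or otherwise clamps the velocity magnitude to a fixed maximum.
; It then calls Jump, releases it with StopJumping after a brief delay and ends; when not on the ground, it ends immediately.
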(event `self.K2_ActivateAbility`
  (bind _charactermovement (`Character.CharacterMovement` (`self.GetPlayerCharacterFromActorInfo`)))
  (set `self.Character Movement` _charactermovement)
  (if (`NavMovementComponent.IsMovingOnGround` _charactermovement)
    (if (== (`KismetMathLibrary.VSize2D` (`WWPlayerController.IsMove` (`self.GetPlayerControllerFromActorInfo`))) 0.0)
      (set `MovementComponent.Velocity` (0.0 0.0 0.0) (`self.Character Movement`))
      (else
        (set `MovementComponent.Velocity` (`KismetMathLibrary.Vector_ClampSizeMax` (`MovementComponent.Velocity` (`self.Character Movement`)) 750.0) (`self.Character Movement`))))
    (`Character.Jump` (`self.GetPlayerCharacterFromActorInfo`))
    (`KismetSystemLibrary.Delay` 0.05)
    (`Character.StopJumping` (`self.GetPlayerCharacterFromActorInfo`))
    (`self.K2_EndAbility`)
    (else
      (`self.K2_EndAbility`))))