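; Gameplay ability that puts the player HUD on screen.
; On activation it creates WBP_PlayerHUD for the owning player controller and adds it to the viewport, without ending the ability in this graph.
; It also defines RotateMoveDirection, not called here, which snaps the character to face its movement input relative to the follow camera's flattened axes.
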(event `self.K2_ActivateAbility`
  (bind _returnvalue (`|CreateWidget` "/Game/_BP/KMJ/Widget/HUD/WBP_PlayerHUD.WBP_PlayerHUD_C" (`self.GetPlayerControllerFromActorInfo`)))
  (`UserWidget.AddToViewport` _returnvalue 0))

(fn `RotateMoveDirection`
  (bind _followcamera (`PlayerCharacter.FollowCamera` (`self.GetPlayerCharacterFromActorInfo`)))
  (bind (_returnvalue_x _returnvalue_y) (`KismetMathLibrary.BreakVector` (`SceneComponent.GetRightVector` _followcamera)))
  (bind (_x _y) (`KismetMathLibrary.BreakVector2D` (`WWPlayerController.IsInputMove` (`self.GetPlayerControllerFromActorInfo`))))
  (bind (_returnvalue_x_2 _returnvalue_y_2) (`KismetMathLibrary.BreakVector` (`SceneComponent.GetForwardVector` _followcamera)))
  (bind _returnvalue (+ (* (`KismetMathLibrary.Normal` (`KismetMathLibrary.MakeVector` _returnvalue_x _returnvalue_y)) _x) (* (`KismetMathLibrary.Normal` (`KismetMathLibrary.MakeVector` _returnvalue_x_2 _returnvalue_y_2)) _y)))
  (if (`KismetMathLibrary.NotEqualExactly_VectorVector` _returnvalue)
    (`Actor.K2_SetActorRotation` (`self.GetPlayerCharacterFromActorInfo`) (`KismetMathLibrary.MakeRotFromX` _returnvalue) true)))