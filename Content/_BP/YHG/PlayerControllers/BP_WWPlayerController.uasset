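; Player controller for a three-character party game (Rover, Chixia, Verina) that handles input, the HUD, weapon inventory, menus and the tower-entry prompt.
; Switching repossesses the chosen pawn, carrying over transform, velocity, modes and control rotation, freezes and hides the old one, and updates tags, HUD and minimap capture.
; A looping timer picks the closest enemy by sphere overlap, retargeting when out of range or dashing with movement input.
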(event `EnhancedInput|/Game/_BP/YHG/Inputs/Actions/IA_Move`
  (params (ActionValue :type "Vector2D Structure") (ElapsedSeconds :type "Float (double-precision)") (TriggeredSeconds :type "Float (double-precision)") (InputAction :type "InputAction Object Reference" :default "/Game/_BP/YHG/Inputs/Actions/IA_Move.IA_Move"))
  (:`Triggered`
    (set `self.IsInputMove` ActionValue))
  (:`Completed`
    (set `self.IsInputMove` (0.0 0.0))))

(event `EnhancedInput|/Game/_BP/YHG/Inputs/Actions/IA_Dash`
  (params (ActionValue :type Boolean) (ElapsedSeconds :type "Float (double-precision)") (TriggeredSeconds :type "Float (double-precision)") (InputAction :type "InputAction Object Reference" :default "/Game/_BP/YHG/Inputs/Actions/IA_Dash.IA_Dash"))
  (:`Started`
    (set `self.bIsInputDash` true)
    (`KismetSystemLibrary.Delay` 0.05)
    (set `self.bIsInputDash` false)))

(event `EnhancedInput|/Game/_BP/YHG/Inputs/Actions/IA_Jump`
  (params (ActionValue :type Boolean) (ElapsedSeconds :type "Float (double-precision)") (TriggeredSeconds :type "Float (double-precision)") (InputAction :type "InputAction Object Reference" :default "/Game/_BP/YHG/Inputs/Actions/IA_Jump.IA_Jump"))
  (:`Started`
    (set `self.bIsInputJump` true)
    (`KismetSystemLibrary.Delay` 0.05)
    (set `self.bIsInputJump` false)))

(event `EnhancedInput|/Game/_BP/YHG/Inputs/Actions/IA_LightAttack`
  (params (ActionValue :type Boolean) (ElapsedSeconds :type "Float (double-precision)") (TriggeredSeconds :type "Float (double-precision)") (InputAction :type "InputAction Object Reference" :default "/Game/_BP/YHG/Inputs/Actions/IA_LightAttack.IA_LightAttack"))
  (:`Started`
    (set `self.bIsInputLightAttack` true)
    (`KismetSystemLibrary.Delay` 0.05)
    (set `self.bIsInputLightAttack` false)))

(event `EnhancedInput|/Game/_BP/YHG/Inputs/Actions/IA_Character1`
  (params (ActionValue :type Boolean) (ElapsedSeconds :type "Float (double-precision)") (TriggeredSeconds :type "Float (double-precision)") (InputAction :type "InputAction Object Reference" :default "/Game/_BP/YHG/Inputs/Actions/IA_Character1.IA_Character1"))
  (bind _widget_playerhud (`self.Widget_PlayerHUD`))
  (bind _widget_playerhud_2 (`self.Widget_PlayerHUD`))
  (bind _wbp_party_icons (`/Game/_BP/KMJ/Widget/HUD/WBP_PlayerHUD.WBP_Party_Icons` _widget_playerhud))
  (:`Triggered`
    (`/Engine/EditorBlueprintResources/StandardMacros.IsValid` _widget_playerhud
      (:`Is Valid`
        (if (not (`/Game/_BP/KMJ/Widget/HUD/Assets/PartyIcon/WBP_HUD_PartyButton.IsCoolTime` (`/Game/_BP/KMJ/Widget/HUD/Assets/WBP_Party_Icons_HUD.WBP_HUD_PartyButton_Rover` _wbp_party_icons)))
          (bind _returnvalue (`GameplayStatics.GetActorOfClass` "/Game/_BP/YHG/Characters/LightRover/BP_LightRoverCharacter.BP_LightRoverCharacter_C"))
          (`/Engine/EditorBlueprintResources/StandardMacros.IsValid` _returnvalue
            (:`Is Valid`
              (if (!= _returnvalue (`self.ControlledPlayerCharacter`))
                (`self.Possess` _returnvalue)
                (`SkeletalMeshComponent.SetAnimInstanceClass` (`Character.Mesh` _returnvalue) "/Game/_BP/YHG/Characters/LightRover/Animation/ABP_LightRoverAnim.ABP_LightRoverAnim_C")
                (`WWBlueprintFunctionLibrary.AddTagToActor` (`self.PlayerState`))
                (`/Game/_BP/KMJ/Widget/HUD/Assets/WBP_Party_Icons_HUD.CharacterChange_Event` _wbp_party_icons "Rover")
                (`self.ChangeMiniMapCamera` true)
                (`/Game/_BP/KMJ/Widget/HUD/WBP_PlayerHUD.LinkPawnToUI` _widget_playerhud_2 "Rover")
                (`/Game/_BP/KMJ/Widget/HUD/Assets/WBP_SkillIcon_E.SetSkillIconByCharacterName` (`/Game/_BP/KMJ/Widget/HUD/WBP_PlayerHUD.WBP_SkillIcon_E_Rover` _widget_playerhud_2) "Rover")))))))))

(event `EnhancedInput|/Game/_BP/YHG/Inputs/Actions/IA_Character2`
  (params (ActionValue :type Boolean) (ElapsedSeconds :type "Float (double-precision)") (TriggeredSeconds :type "Float (double-precision)") (InputAction :type "InputAction Object Reference" :default "/Game/_BP/YHG/Inputs/Actions/IA_Character2.IA_Character2"))
  (bind _widget_playerhud (`self.Widget_PlayerHUD`))
  (bind _widget_playerhud_2 (`self.Widget_PlayerHUD`))
  (bind _wbp_party_icons (`/Game/_BP/KMJ/Widget/HUD/WBP_PlayerHUD.WBP_Party_Icons` _widget_playerhud))
  (:`Triggered`
    (`/Engine/EditorBlueprintResources/StandardMacros.IsValid` _widget_playerhud
      (:`Is Valid`
        (if (not (`/Game/_BP/KMJ/Widget/HUD/Assets/PartyIcon/WBP_HUD_PartyButton.IsCoolTime` (`/Game/_BP/KMJ/Widget/HUD/Assets/WBP_Party_Icons_HUD.WBP_HUD_PartyButton_Chixia` _wbp_party_icons)))
          (bind _returnvalue (`GameplayStatics.GetActorOfClass` "/Game/_BP/YHG/Characters/Chixia/BP_ChixiaCharacter.BP_ChixiaCharacter_C"))
          (`/Engine/EditorBlueprintResources/StandardMacros.IsValid` _returnvalue
            (:`Is Valid`
              (if (!= _returnvalue (`self.ControlledPlayerCharacter`))
                (`self.Possess` _returnvalue)
                (`SkeletalMeshComponent.SetAnimInstanceClass` (`Character.Mesh` _returnvalue) "/Game/_BP/YHG/Characters/Chixia/Animation/ABP_ChixiaAnim.ABP_ChixiaAnim_C")
                (`/Game/_BP/KMJ/Widget/HUD/Assets/WBP_Party_Icons_HUD.CharacterChange_Event` _wbp_party_icons "Chixia")
                (`self.ChangeMiniMapCamera` false true)
                (`/Game/_BP/KMJ/Widget/HUD/WBP_PlayerHUD.LinkPawnToUI` _widget_playerhud_2 "Chixia")
                (`/Game/_BP/KMJ/Widget/HUD/Assets/WBP_SkillIcon_E.SetSkillIconByCharacterName` (`/Game/_BP/KMJ/Widget/HUD/WBP_PlayerHUD.WBP_SkillIcon_E_Rover` _widget_playerhud_2) "Chixia")))))))))

(event `EnhancedInput|/Game/_BP/YHG/Inputs/Actions/IA_Character3`
  (params (ActionValue :type Boolean) (ElapsedSeconds :type "Float (double-precision)") (TriggeredSeconds :type "Float (double-precision)") (InputAction :type "InputAction Object Reference" :default "/Game/_BP/YHG/Inputs/Actions/IA_Character3.IA_Character3"))
  (bind _widget_playerhud (`self.Widget_PlayerHUD`))
  (bind _widget_playerhud_2 (`self.Widget_PlayerHUD`))
  (bind _wbp_party_icons (`/Game/_BP/KMJ/Widget/HUD/WBP_PlayerHUD.WBP_Party_Icons` _widget_playerhud))
  (:`Triggered`
    (`/Engine/EditorBlueprintResources/StandardMacros.IsValid` _widget_playerhud
      (:`Is Valid`
        (if (not (`/Game/_BP/KMJ/Widget/HUD/Assets/PartyIcon/WBP_HUD_PartyButton.IsCoolTime` (`/Game/_BP/KMJ/Widget/HUD/Assets/WBP_Party_Icons_HUD.WBP_HUD_PartyButton_Verina` _wbp_party_icons)))
          (bind _returnvalue (`GameplayStatics.GetActorOfClass` "/Game/_BP/YHG/Characters/Verina/BP_VerinaCharacter.BP_VerinaCharacter_C"))
          (`/Engine/EditorBlueprintResources/StandardMacros.IsValid` _returnvalue
            (:`Is Valid`
              (if (!= _returnvalue (`self.ControlledPlayerCharacter`))
                (`self.Possess` _returnvalue)
                (`SkeletalMeshComponent.SetAnimInstanceClass` (`Character.Mesh` _returnvalue) "/Game/_BP/YHG/Characters/Verina/Animation/ABP_VerinaAnim.ABP_VerinaAnim_C")
                (`/Game/_BP/KMJ/Widget/HUD/Assets/WBP_Party_Icons_HUD.CharacterChange_Event` _wbp_party_icons "Verina")
                (`self.ChangeMiniMapCamera` false false true)
                (`/Game/_BP/KMJ/Widget/HUD/WBP_PlayerHUD.LinkPawnToUI` _widget_playerhud_2 "Verina")
                (`/Game/_BP/KMJ/Widget/HUD/Assets/WBP_SkillIcon_E.SetSkillIconByCharacterName` (`/Game/_BP/KMJ/Widget/HUD/WBP_PlayerHUD.WBP_SkillIcon_E_Rover` _widget_playerhud_2) "Verina")))))))))

(event `self.ReceiveUnPossess`
  (params (UnpossessedPawn :type "Pawn Object Reference"))
  (set `self.Unpossessed Pawn` UnpossessedPawn)
  (set `self.OldRotation` (`self.GetControlRotation`)))

(event `self.ReceivePossess`
  (params (PossessedPawn :type "Pawn Object Reference"))
  (bind _playerstate (`self.PlayerState`))
  (bind _playerstate_2 (`self.PlayerState`))
  (bind _playerstate_3 (`self.PlayerState`))
  (set `self.Possessed Pawn` PossessedPawn)
  (`|ExecutionSequence`
    (:`then_0`
      (bind _asbp_light_rover_character (cast `/Game/_BP/YHG/Characters/LightRover/BP_LightRoverCharacter` (`self.Possessed Pawn`)))
      (`/Game/_BP/YHG/Characters/LightRover/BP_LightRoverCharacter.CheckFirstPossessAndInitialize` _asbp_light_rover_character)
      (`WWBlueprintFunctionLibrary.AddTagToActor` _playerstate_3 (struct :`TagName` "Player.Status.PlayingCharacter.LightRover"))
      (`WWBlueprintFunctionLibrary.RemoveTagFromActor` _playerstate_3 (struct :`TagName` "Player.Status.PlayingCharacter.Chixia"))
      (`WWBlueprintFunctionLibrary.RemoveTagFromActor` _playerstate_3 (struct :`TagName` "Player.Status.PlayingCharacter.Verina")))
    (:`then_1`
      (bind _asbp_chixia_character (cast `/Game/_BP/YHG/Characters/Chixia/BP_ChixiaCharacter` (`self.Possessed Pawn`)))
      (`/Game/_BP/YHG/Characters/Chixia/BP_ChixiaCharacter.CheckFirstPossessAndInitialize` _asbp_chixia_character)
      (`WWBlueprintFunctionLibrary.AddTagToActor` _playerstate (struct :`TagName` "Player.Status.PlayingCharacter.Chixia"))
      (`WWBlueprintFunctionLibrary.RemoveTagFromActor` _playerstate (struct :`TagName` "Player.Status.PlayingCharacter.LightRover"))
      (`WWBlueprintFunctionLibrary.RemoveTagFromActor` _playerstate (struct :`TagName` "Player.Status.PlayingCharacter.Verina")))
    (:`then_2`
      (bind _asbp_verina_character (cast `/Game/_BP/YHG/Characters/Verina/BP_VerinaCharacter` (`self.Possessed Pawn`)))
      (`/Game/_BP/YHG/Characters/Verina/BP_VerinaCharacter.CheckFirstPossessAndInitialize` _asbp_verina_character)
      (`WWBlueprintFunctionLibrary.AddTagToActor` _playerstate_2 (struct :`TagName` "Player.Status.PlayingCharacter.Verina"))
      (`WWBlueprintFunctionLibrary.RemoveTagFromActor` _playerstate_2 (struct :`TagName` "Player.Status.PlayingCharacter.LightRover"))
      (`WWBlueprintFunctionLibrary.RemoveTagFromActor` _playerstate_2 (struct :`TagName` "Player.Status.PlayingCharacter.Chixia")))
    (:`then_3`
      (bind _asbp_player_character (cast `/Game/_BP/YHG/Characters/BP_PlayerCharacter` (`self.Unpossessed Pawn`)))
      (set `self.CachedPawnVelocity` (`MovementComponent.Velocity` (`Character.CharacterMovement` _asbp_player_character)))
      (set `self.CachedSprintMode` (`PlayerCharacter.bSprintMode` _asbp_player_character))
      (set `self.CachedAttackMode` (`PlayerCharacter.bAttackMode` _asbp_player_character))
      (`self.SetActorHiddenInGame` _asbp_player_character true)
      (`self.SetActorEnableCollision` _asbp_player_character false)
      (`self.SetActorTickEnabled` _asbp_player_character false)
      (set `Actor.CustomTimeDilation` 0.0 _asbp_player_character)
      (bind _asbp_player_character_2 (cast `/Game/_BP/YHG/Characters/BP_PlayerCharacter` (`self.Possessed Pawn`)))
      (set `MovementComponent.Velocity` (`self.CachedPawnVelocity`) (`Character.CharacterMovement` _asbp_player_character_2))
      (set `PlayerCharacter.bSprintMode` (`self.CachedSprintMode`) _asbp_player_character_2)
      (set `PlayerCharacter.bAttackMode` (`self.CachedAttackMode`) _asbp_player_character_2)
      (`self.K2_SetActorLocationAndRotation` _asbp_player_character_2 (`self.K2_GetActorLocation` _asbp_player_character) (`self.K2_GetActorRotation` _asbp_player_character) false false)
      (`self.SetActorHiddenInGame` _asbp_player_character_2 false)
      (`self.SetActorEnableCollision` _asbp_player_character_2 true)
      (`self.SetActorTickEnabled` _asbp_player_character_2 true)
      (set `Actor.CustomTimeDilation` 1.0 _asbp_player_character_2))
    (:`then_4`
      (`self.SetControlRotation` (`self.OldRotation`)))))

(event `self.ReceiveBeginPlay`
  (`KismetSystemLibrary.K2_SetTimer` null "FindClosestEnemy" 0.1 true)
  (`KismetArrayLibrary.Array_Clear` (`self.Inventory_Weapon`))
  (bind _outrownames (`DataTableFunctionLibrary.GetDataTableRowNames` "/Game/_BP/KMJ/DataTable/Weapons/DT_Inventory_Weapon.DT_Inventory_Weapon"))
  (for _array_element _outrownames
    (bind _returnvalue (`|GetDataTableRow` "/Game/_BP/KMJ/DataTable/Weapons/DT_Inventory_Weapon.DT_Inventory_Weapon" _array_element)
      (:`then`
        (`KismetArrayLibrary.Array_Add` (`self.Inventory_Weapon`) _returnvalue))))
  (bind _returnvalue_2 (`WeaponSkillDataHelper.WeaponSortByStandard` (`self.Weapon Data`) (`self.Inventory_Weapon`) "Rarity"))
  (`KismetArrayLibrary.Array_Clear` (`self.Inventory_Weapon`))
  (set `self.Inventory_Weapon` _returnvalue_2)
  (bind _returnvalue_3 (`|CreateWidget` "/Game/_BP/KMJ/Widget/HUD/WBP_PlayerHUD.WBP_PlayerHUD_C"))
  (`WWUserWidget.InitHUDSharedWidget` _returnvalue_3 self)
  (bind _output_get (set `self.Widget_PlayerHUD` _returnvalue_3))
  (`UserWidget.AddToViewport` _output_get 0)
  (bind _returnvalue_4 (`GameplayStatics.GetActorOfClass` "/Game/_BP/YHG/Characters/LightRover/BP_LightRoverCharacter.BP_LightRoverCharacter_C"))
  (set `self.Character_Rover` _returnvalue_4)
  (bind _returnvalue_5 (`GameplayStatics.GetActorOfClass` "/Game/_BP/YHG/Characters/Chixia/BP_ChixiaCharacter.BP_ChixiaCharacter_C"))
  (set `self.Character_Chixia` _returnvalue_5)
  (bind _returnvalue_6 (`GameplayStatics.GetActorOfClass` "/Game/_BP/YHG/Characters/Verina/BP_VerinaCharacter.BP_VerinaCharacter_C"))
  (set `self.Character_Verina` _returnvalue_6)
  (`self.ChangeMiniMapCamera` true)
  (`/Game/_BP/KMJ/Widget/HUD/WBP_PlayerHUD.LinkPawnToUI` (`self.Widget_PlayerHUD`) "Rover")
  (bind _asbp_game_instance (cast `/Game/_BP/Common/GameInstance/BP_GameInstance` (`GameplayStatics.GetGameInstance`)))
  (if (`WWGameInstance.bIsSaveDataExist` _asbp_game_instance)
    (`/Game/_BP/Common/GameInstance/BP_GameInstance.LoadAllDataAfterChangeLevel` _asbp_game_instance)))

(event `/Game/_BP/KMJ/Interface/BPI_ChangeWeapon.ChangeWeapon`
  (params (PreviousWeapon :type "Inventory_Weapon Structure") (NewWeapon :type "Inventory_Weapon Structure") (Index :type Integer))
  (`self.ChangeEquippedWeapon` PreviousWeapon NewWeapon Index))

(event `Key|C`
  (params (Key :type "Key Structure"))
  (:`Pressed`
    (`/Game/_BP/KMJ/Widget/CharacterSetting/BP_CharSettingUIComponent.CreateWidget_CharSetting` (`self.BP_CharSettingUIComponent`))
    (`Widget.SetVisibility` (`self.Widget_PlayerHUD`) "Hidden")
    (`GameplayStatics.SetGamePaused` true)))

(event `Key|B`
  (params (Key :type "Key Structure"))
  (:`Pressed`
    (`/Game/_BP/KMJ/Widget/CharacterSetting/BP_CharSettingUIComponent.CreateWidget_Inventory` (`self.BP_CharSettingUIComponent`))
    (`Widget.SetVisibility` (`self.Widget_PlayerHUD`) "Hidden")
    (`GameplayStatics.SetGamePaused` true)))

(event `self.ReceiveTick`
  (params (DeltaSeconds :type "Float (single-precision)")))

(event `Key|F`
  (params (Key :type "Key Structure"))
  (:`Pressed`
    (if (`self.Is Tower Enter Enable`)
      (bind _returnvalue (`|CreateWidget` "/Game/_BP/KMJ/Widget/Tower/WBP_Tower_Intro.WBP_Tower_Intro_C" self))
      (`UserWidget.AddToViewport` _returnvalue 0)
      (`WidgetBlueprintLibrary.SetInputMode_UIOnlyEx` self null)
      (set `self.bShowMouseCursor` true))))

(event `/Game/_BP/KMJ/Interface/BPI_ReloadInventory.ReloadInventory`
  (params (Sort :type "EWeaponSortStandard Enum" :default "Rarity"))
  (`KismetArrayLibrary.Array_Clear` (`self.CachedWeapon`))
  (switch `EWeaponSortStandard` Sort
    (:`Rarity`
      (bind _returnvalue (`WeaponSkillDataHelper.WeaponSortByStandard` (`self.Weapon Data`) (`self.Inventory_Weapon`) Sort :!label _label))
      (set `self.CachedWeapon` _returnvalue))
    (:`Level`
      (goto _label))
    (:`Reverse`
      (`KismetArrayLibrary.Array_Reverse` (`self.Inventory_Weapon`))
      (set `self.CachedWeapon` (`self.Inventory_Weapon`))))
  (`KismetArrayLibrary.Array_Clear` (`self.Inventory_Weapon`))
  (set `self.Inventory_Weapon` (`self.CachedWeapon`)))

(fn `ChangeEquippedWeapon`
  (params (PreviousWeapon :type "Inventory_Weapon Structure") (NewWeapon :type "Inventory_Weapon Structure") (Index :type Integer))
  (bind (_weaponcurrentlevel _weaponcurrentrank _skillrank _itemowner _itemownerimage _rowindex) (break `Inventory_Weapon` NewWeapon))
  (bind (_weaponcurrentlevel_2 _weaponcurrentrank_2 _skillrank_2 _itemowner_2 _itemownerimage_2) (break `Inventory_Weapon` PreviousWeapon))
  ;[0.2969 0.2969 0.2969] 무기 장착 해제
  (for (_array_element _array_index) (`self.Inventory_Weapon`)
    (bind (_weaponcurrentlevel_3 _weaponcurrentrank_3 _skillrank_3 _itemowner_3 _itemownerimage_3 _rowindex_2) (break `Inventory_Weapon` _array_element))
    (if (`|EnumEquality` _itemowner_3 _itemowner_2)
      (`KismetArrayLibrary.Array_Set` (`self.Inventory_Weapon`) _array_index (make `Inventory_Weapon` _weaponcurrentlevel_3 _weaponcurrentrank_3 _skillrank_3 "None" _itemownerimage_3 _rowindex_2))
      (break)))
  ;[0.2708 0.2708 0.2708] 무기 새로 장착
  (for (_ _array_index_2) (`self.Inventory_Weapon`)
    (if (== Index _array_index_2)
      (`KismetArrayLibrary.Array_Set` (`self.Inventory_Weapon`) _array_index_2 (make `Inventory_Weapon` _weaponcurrentlevel _weaponcurrentrank _skillrank _itemowner_2 _itemownerimage_2 _rowindex))
      (break))))

(fn `ChangeMiniMapCamera`
  (params (Rover :type Boolean) (Chixia :type Boolean) (Verina :type Boolean))
  (`SceneComponent.SetVisibility` (`/Game/_BP/YHG/Characters/LightRover/BP_LightRoverCharacter.SceneCaptureComponent2D` (`self.Character_Rover`)) Rover true)
  (`SceneComponent.SetVisibility` (`/Game/_BP/YHG/Characters/Chixia/BP_ChixiaCharacter.SceneCaptureComponent2D` (`self.Character_Chixia`)) Chixia true)
  (`SceneComponent.SetVisibility` (`/Game/_BP/YHG/Characters/Verina/BP_VerinaCharacter.SceneCaptureComponent2D` (`self.Character_Verina`)) Verina true))

(fn `FindClosestEnemy`
  (locals (`Object Types` :type "Array of EObjectTypeQuery Enum") (DetectMonsters :type "Array of Actor Object Reference"))
  (bind _controlledplayercharacter (`self.ControlledPlayerCharacter`))
  (bind _outactors (`KismetSystemLibrary.SphereOverlapActors` (`self.K2_GetActorLocation` (`self.ControlledPlayerCharacter`)) 768.0 (`local.Object Types`) "/Script/WutheringWaves.EnemyCharacter"))
  (bind _output_get (set `local.DetectMonsters` _outactors))
  (if (`KismetArrayLibrary.Array_IsEmpty` _output_get)
    (set `self.ClosestEnemy` null)
    (else
      ;[1 1 1] 조우 시에는 대쉬없어도 타겟 잡기
      (`/Engine/EditorBlueprintResources/StandardMacros.IsValid` (`self.ClosestEnemy`)
        (:`Is Valid`
          (if (> (`KismetMathLibrary.VSize` (- (`self.K2_GetActorLocation` (`self.ControlledPlayerCharacter`)) (`self.K2_GetActorLocation` (`self.ClosestEnemy`)))) 768.0)
            (set `self.ClosestEnemy` (`.ReturnValue` (`GameplayStatics.FindNearestActor` (`self.K2_GetActorLocation` (`self.ControlledPlayerCharacter`)) (`local.DetectMonsters`))))
            (else
              (`WWBlueprintFunctionLibrary.BP_HasTag` _controlledplayercharacter (struct :`TagName` "Player.Status.Dashing")
                (:`Yes`
                  (if (> (`KismetMathLibrary.VSize2D` (`self.IsInputMove`)) 0.0)
                    (set `self.ClosestEnemy` (`.ReturnValue` (`GameplayStatics.FindNearestActor` (`self.K2_GetActorLocation` _controlledplayercharacter) (`local.DetectMonsters`))))))))))
        (:`Is Not Valid`
          (set `self.ClosestEnemy` (`.ReturnValue` (`GameplayStatics.FindNearestActor` (`self.K2_GetActorLocation` (`self.ControlledPlayerCharacter`)) (`local.DetectMonsters`)))))))))

(fn `IsTowerEnterEnable`
  (params (bIsTowerEnterEnable :type Boolean))
  (bind _wbp_fkey (`/Game/_BP/KMJ/Widget/HUD/WBP_PlayerHUD.WBP_FKey` (`self.Widget_PlayerHUD`)))
  (bind _output_get (set `self.Is Tower Enter Enable` bIsTowerEnterEnable))
  (if _output_get
    (`Widget.SetVisibility` _wbp_fkey "Visible")
    (else
      (`Widget.SetVisibility` _wbp_fkey "Hidden"))))

(fn `UserConstructionScript`)